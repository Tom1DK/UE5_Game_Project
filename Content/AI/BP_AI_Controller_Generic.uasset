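; Generic AI controller that runs the BT_AI behavior tree and feeds it perception results from sight and hearing.
; Perception updates run both detection functions, which write blackboard keys.
; A successful sighting sets Target_Actor; lost sight or any non-sight stimulus, including hearing, clears it.
; Hearing stimuli set Investigation_Location and enable the investigation icon on the controlled BP_AI pawn.
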(event OnTargetPerceptionUpdated(AIPerception)
  (params (Actor :type Actor%20Object%20Reference) (Stimulus :type AI%20Stimulus%20Structure))
  ;[1 1 1] Detect and Chase/Investigate Targets
  (CallFunction|SightDetection Actor Stimulus)
  (CallFunction|HearingDetection Actor Stimulus))

(event EventBeginPlay
  (AI|RunBehaviorTree "/Game/AI/BT_AI.BT_AI"))

(fn ConstructionScript)

(fn SightDetection
  (params (actor :type Actor%20Object%20Reference) (stimulus :type AI%20Stimulus%20Structure))
  ;[1 1 1] Detect and Chase Target
  (bind _returnvalue (Class|AIPerceptionSystem|GetSenseClassforStimulus stimulus))
  (if (== _returnvalue "/Script/AIModule.AISense_Sight")
    (if (.bSuccessfullySensed (Utilities|Struct|BreakAIStimulus stimulus))
      (AI|Components|Blackboard|SetValueasObject (AI|GetBlackboard 0) (Utilities|Name|MakeLiteralName "Target_Actor") actor)
      (else
        (AI|Components|Blackboard|SetValueasObject (AI|GetBlackboard 0) (Utilities|Name|MakeLiteralName "Target_Actor") 0 :!label _label)))
    (else
      (goto _label))))

(fn HearingDetection
  (params (actor :type Actor%20Object%20Reference) (Stimulus :type AI%20Stimulus%20Structure))
  (bind _returnvalue (Class|AIPerceptionSystem|GetSenseClassforStimulus Stimulus))
  (if (== _returnvalue "/Script/AIModule.AISense_Hearing")
    (AI|Components|Blackboard|SetValueasVector (AI|GetBlackboard 0) (Utilities|Name|MakeLiteralName "Investigation_Location") (.StimulusLocation (Utilities|Struct|BreakAIStimulus Stimulus)))
    (bind _asbp_ai (Utilities|Casting|CastToBP_AI (Pawn|GetControlledPawn)))
    (Default|EnableInvestigationIcon _asbp_ai)))