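; Enemy AI character with melee attacks, hit reactions, ragdoll death and a stealth back-assassination prompt for the player.
; Attack feeds an indexed montage combo that queues follow-up swings, with timer-looped sword traces and a sphere trace damaging "Damagable" actors.
; Damage plays a random hit montage, launches it along the player's facing and updates BPCPlayerStats, which triggers ragdoll.
; Tick turns the health bar and assassination widgets toward the camera.
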(event OnComponentBeginOverlap(AssassinationRadius)
  (params (OverlappedComponent :type Primitive%20Component%20Object%20Reference) (OtherActor :type Actor%20Object%20Reference) (OtherComp :type Primitive%20Component%20Object%20Reference) (OtherBodyIndex :type Integer) (bFromSweep :type Boolean) (SweepResult :type Hit%20Result%20Structure%20%28by%20ref%29))
  (Utilities|Casting|CastToBP_ThirdPersonCharacter OtherActor)
  (Rendering|SetVisibility (Variables|Default|GetAssassinate_Widget) true false))

(event OnComponentEndOverlap(AssassinationRadius)
  (params (OverlappedComponent :type Primitive%20Component%20Object%20Reference) (OtherActor :type Actor%20Object%20Reference) (OtherComp :type Primitive%20Component%20Object%20Reference) (OtherBodyIndex :type Integer))
  (Utilities|Casting|CastToBP_ThirdPersonCharacter OtherActor)
  (Rendering|SetVisibility (Variables|Default|GetAssassinate_Widget) false false))

(event Custom|Sword_Attack
  ;[1 1 1] Combo System
  ;;[1 1 1] Sword Attack
  (if (Variables|Default|Getis_attacking?)
    (Variables|Default|Setsave_attack? true)
    (else
      (Variables|Default|Setis_attacking? true)
      (switch int (Variables|Default|Getattack_index)
        (:0
          (CallFunction|Attack1))
        (:1
          (CallFunction|Attack2))
        (:2
          (CallFunction|Attack3))
        (:3
          (CallFunction|Attack4))))))

(event Custom|Sword_Attack_Combo
  ;[1 1 1] Combo System
  ;;[1 1 1] Combo Count
  (if (Variables|Default|Getsave_attack?)
    (Variables|Default|Setsave_attack? false)
    (switch int (Variables|Default|Getattack_index)
      (:0
        (CallFunction|Attack1))
      (:1
        (CallFunction|Attack2))
      (:2
        (CallFunction|Attack3))
      (:3
        (CallFunction|Attack4)))
    (else
      (CallFunction|StopCombo))))

(event Custom|Attack_2
  ;[1 1 1] Combo System
  ;;[1 1 1] Attack 2
  (Utilities|FlowControl|DoOnce false :!label _label
    (:Completed
      (Utilities|FlowControl|Delay 0.5)
      (Animation|Montage|PlayMontage (Variables|Character|GetMesh) "/Game/Characters/RPG_Character/Animations/Sword_Attacks/Attack2_Montage.Attack2_Montage"
        (:then
          (Variables|Default|Setattack_index 2)
          (goto _label Reset))))))

(event Custom|Play_Sword_Hit_Sound
  ;[1 1 1] Sound Effects
  (Audio|PlaySoundatLocation "/Game/Audio/Sword-Hits/MS_Sword_Hit.MS_Sword_Hit" (Transformation|GetActorLocation (Components|GetOwner)) "0, 0, 0" 1.0 1.0 0.0 0 0 0 0))

(event Custom|Attack_3
  ;[1 1 1] Combo System
  ;;[1 1 1] Attack 3 (Not Being Used ATM)
  (Utilities|FlowControl|DoOnce false :!label _label
    (:Completed
      (Utilities|FlowControl|Delay 0.45)
      (Animation|Montage|PlayMontage (Variables|Character|GetMesh) "/Game/Characters/RPG_Character/Animations/Sword_Attacks/Kick_Montage.Kick_Montage"
        (:then
          (Variables|Default|Setattack_index 3)
          (goto _label Reset))))))

(event Custom|Sword%20Attack/Combo%20Call%20From%20BT
  ;[1 1 1] Combo System
  ;;[1 1 1] Attack Input
  (if (Variables|Default|Getcan_attack?)
    (CallFunction|SwordAttack)))

(event Custom|Ragdoll
  ;[1 1 1] Ragdoll
  (Utilities|FlowControl|Sequence
    (:then_0
      (Utilities|FlowControl|Delay 2.5)
      (Physics|SetSimulatePhysics (Variables|Character|GetMesh) true))
    (:then_1
      (Utilities|FlowControl|Delay 2.2)
      (Audio|PlaySoundatLocation "/Game/Audio/Grunts-Hits/SC_Death.SC_Death" (Transformation|GetActorLocation) "0, 0, 0" 1.0 1.0 0.0 "/Game/Audio/SA_Character.SA_Character" 0 0 0))))

(event Custom|Stop_Combo
  ;[1 1 1] Combo System
  ;;[1 1 1] Stop Combo/Attack
  (Variables|Default|Setis_attacking? false)
  (Variables|Default|Setattack_index 0))

(event Custom|Attack_4
  ;[1 1 1] Combo System
  ;;[1 1 1] Attack 4
  (Utilities|FlowControl|DoOnce false :!label _label
    (:Completed
      (Utilities|FlowControl|Delay 0.4)
      (Animation|Montage|PlayMontage (Variables|Character|GetMesh) "/Game/Characters/RPG_Character/Animations/Sword_Attacks/Attack3_Montage.Attack3_Montage"
        (:then
          (Variables|Default|Setattack_index 4)
          (goto _label Reset))))))

(event Custom|Start_Sword_Trace
  ;[1 1 1] Sword Trace 1/4
  (bind _returnvalue (Utilities|Time|SetTimerbyEvent (delegate Custom|Sword_Trace_Loop) 0.01 true))
  (Variables|Default|Setsword_trace_loop_var _returnvalue))

(event Custom|Sword_Trace_Loop
  ;[1 1 1] Sword Trace 1/4
  (bind (_outhit _returnvalue) (Collision|SphereTraceByChannel (Transformation|GetWorldLocation (Variables|Default|GetWeapon%20Top%20Point)) (Transformation|GetWorldLocation (Variables|Default|GetWeapon%20Bottom%20Point)) 12.0 "TraceTypeQuery1" false 0 "ForDuration" true "(R=1.000000,G=0.000000,B=0.000000,A=1.000000)" "(R=0.000000,G=1.000000,B=0.000000,A=1.000000)" 1.0))
  (if _returnvalue
    (if (Actor|ActorHasTag (.HitActor (Collision|BreakHitResult _outhit)) "Damagable")
      (Utilities|FlowControl|DoOnce false :!label _label
        (:Completed
          (Game|Damage|ApplyDamage (.HitActor (Collision|BreakHitResult _outhit)) 2.0 0 0)
          (Camera|PlayWorldCameraShake "/Game/Blueprints/BP_Sword_Hit_Camera_Shake.BP_Sword_Hit_Camera_Shake_C" (.Location (Collision|BreakHitResult _outhit)) 0.0 2e+03)
          (CallFunction|PlaySwordHitSound)
          (Effects|SpawnEmitteratLocation "/Game/VFX/Particles/Blood/P_Blood_Splat_Cone.P_Blood_Splat_Cone" (.Location (Collision|BreakHitResult _outhit)) (Math|Rotator|MakeRotfromXY (.Normal (Collision|BreakHitResult _outhit)) (.Normal (Collision|BreakHitResult _outhit))) "2.000000,2.000000,2.000000" true "AutoRelease")
          (Utilities|FlowControl|Delay 0.5)
          (goto _label Reset))))))

(event Custom|Stop_Sword_Trace
  ;[1 1 1] Sword Trace 1/4
  (Utilities|Time|ClearandInvalidateTimerbyHandle (Variables|Default|Getsword_trace_loop_var)))

(event Custom|Sphere_Trace
  (bind _sphere_trace (Variables|Default|GetSphere%20Trace))
  (bind _returnvalue (Transformation|GetWorldLocation _sphere_trace))
  ;[1 1 1] Sphere Trace (For Stab and Kick) 2/3
  (bind (_outhit _returnvalue_2) (Collision|SphereTraceByChannel _returnvalue _returnvalue 45.0 "TraceTypeQuery1" false 0 "ForDuration" true "(R=1.000000,G=0.000000,B=0.000000,A=1.000000)" "(R=0.000000,G=1.000000,B=0.000000,A=1.000000)" 1.0))
  (if _returnvalue_2
    (if (Actor|ActorHasTag (.HitActor (Collision|BreakHitResult _outhit)) "Damagable")
      (Game|Damage|ApplyDamage (.HitActor (Collision|BreakHitResult _outhit)) 1.0 0 0)
      (Camera|PlayWorldCameraShake "/Game/Blueprints/BP_Sword_Hit_Camera_Shake.BP_Sword_Hit_Camera_Shake_C" (.Location (Collision|BreakHitResult _outhit)) 0.0 2e+03)
      (CallFunction|KickHitSound)
      (Effects|SpawnEmitteratLocation "/Game/VFX/Particles/Blood/P_Blood_Splat_Cone.P_Blood_Splat_Cone" (.Location (Collision|BreakHitResult _outhit)) (Math|Rotator|MakeRotfromXY (.Normal (Collision|BreakHitResult _outhit)) (.Normal (Collision|BreakHitResult _outhit))) "2.000000,2.000000,2.000000" true "AutoRelease"))))

(event Custom|Attack_1
  ;[1 1 1] Combo System
  ;;[1 1 1] Attack 1
  (Utilities|FlowControl|DoOnce false :!label _label
    (:Completed
      (Utilities|FlowControl|Delay 0.1)
      (Animation|Montage|PlayMontage (Variables|Character|GetMesh) "/Game/Characters/RPG_Character/Animations/Sword_Attacks/Attack1_Montage.Attack1_Montage"
        (:then
          (Variables|Default|Setattack_index 1)
          (goto _label Reset))))))

(event Custom|Kick_Hit_sound
  ;[1 1 1] Sound Effects
  (Audio|PlaySoundatLocation "/Game/Audio/Sword-Hits/Kick.Kick" (Transformation|GetActorLocation (Components|GetOwner)) "0, 0, 0" 1.0 1.0 0.0 0 0 0 0))

(event EventBeginPlay
  (bind _aswb_dummy_healthbar (Utilities|Casting|CastToWB_Dummy_Healthbar (UserInterface|GetWidget (Variables|Default|GetHealth_Bar_Widget))))
  (Variables|Default|Sethealth_bar_ui _aswb_dummy_healthbar))

(event EventTick
  (params (DeltaSeconds :type Float%20%28single-precision%29))
  (Transformation|SetWorldRotation (Variables|Default|GetAssassinate_Widget) (Math|Rotator|FindLookatRotation (Transformation|GetWorldLocation (Variables|Default|GetAssassinate_Widget)) (Transformation|GetWorldLocation (Variables|/Script/Engine.PlayerCameraManager|GetTransformComponent (Game|GetPlayerCameraManager 0)))) false false))

(event Game|Damage|EventAnyDamage
  (params (Damage :type Float%20%28single-precision%29) (DamageType :type Damage%20Type%20Object%20Reference) (InstigatedBy :type Controller%20Object%20Reference) (DamageCauser :type Actor%20Object%20Reference))
  (Animation|PlayAnimMontage (Utilities|Array|Get(acopy) (Variables|Default|Gethit_anims) (Math|Random|RandomIntegerinRange 0 (- (Utilities|Array|Length (Variables|Default|Gethit_anims)) 1))) 1.0 "None")
  (bind _asbp_third_person_character (Utilities|Casting|CastToBP_ThirdPersonCharacter (Game|GetPlayerCharacter 0)))
  (Character|LaunchCharacter (* (Math|Vector|GetForwardVector (Transformation|GetActorRotation _asbp_third_person_character)) 7e+02) false false)
  (Audio|PlaySoundatLocation "/Game/Audio/Grunts-Hits/Death2.Death2" (Transformation|GetActorLocation) "0, 0, 0" 1.0 (Math|Random|RandomFloatinRange 0.8 1.0) 0.0 "/Game/Audio/SA_Character.SA_Character" 0 0 0)
  (bind _is_player_dead (Default|DecreaseHealth (Variables|Default|GetBPC_Player_Stats) Damage))
  (if _is_player_dead
    (Collision|SetCollisionObjectType (Variables|Character|GetMesh) "ECC_PhysicsBody")
    (Physics|SetSimulatePhysics (Variables|Character|GetMesh) true)
    (Audio|PlaySoundatLocation "/Game/Audio/Grunts-Hits/SC_Death.SC_Death" (Transformation|GetActorLocation) "0, 0, 0" 1.0 1.0 0.0 "/Game/Audio/SA_Character.SA_Character" 0 0 0)
    (Rendering|SetVisibility (Variables|Default|GetHealth_Bar_Widget) false false)))

(fn ConstructionScript)

(fn Attack
  (CallFunction|SwordAttack/ComboCallfromBT)
  (return 0.4))

(fn StealthBackAssassination
  (Animation|PlayAnimMontage "/Game/Characters/RPG_Character/Animations/Assassinations/Paired_Knife_Stealth_KidneyAndNeck_Vic_Montage.Paired_Knife_Stealth_KidneyAndNeck_Vic_Montage" 1.0 "None")
  (CallFunction|Ragdoll)
  (Rendering|SetVisibility (Variables|Default|GetAssassinate_Widget) false false)
  (return (Transformation|GetWorldLocation (Variables|Default|GetAssassin_REF)) (Transformation|GetActorRotation)))