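; BP_AI_Boss is the boss AI actor, which feeds its health state to its AI controller.
; Every Tick, after the parent Tick, it casts its controller to BP_AI_Controller_Boss.
; It then copies current and max health from the BPCPlayerStats component into that controller, polling rather than reacting to change events.
; BeginPlay is disabled and the construction script only calls its parent.
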(event EventBeginPlay
  (|CallParentFunction) ; This node is disabled and will not be called.\nDrag off pins to build functionality.
)

(event Collision|EventActorBeginOverlap
  (params (OtherActor :type Actor%20Object%20Reference)))

(event EventTick
  (params (DeltaSeconds :type Float%20%28single-precision%29))
  (bind _bpc_player_stats (Variables|Default|GetBPC_Player_Stats))
  (|CallParentFunction DeltaSeconds)
  (bind _asbp_ai_controller_boss (Utilities|Casting|CastToBP_AI_Controller_Boss (AI|GetAIController self)))
  (Variables|/Game/AI/Boss/BP_AI_Controller_Boss.BP_AI_Controller_Boss_C|Sethealth _asbp_ai_controller_boss (Variables|/Game/Blueprints/BPC_Player_Stats.BPC_Player_Stats_C|GetCurrent_Health _bpc_player_stats))
  (Variables|/Game/AI/Boss/BP_AI_Controller_Boss.BP_AI_Controller_Boss_C|Setmax_health _asbp_ai_controller_boss (Variables|/Game/Blueprints/BPC_Player_Stats.BPC_Player_Stats_C|GetMax_Health _bpc_player_stats)))

(fn ConstructionScript
  (|CallParentFunction))