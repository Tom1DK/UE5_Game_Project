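; Boss AI controller that runs the boss behavior tree on BeginPlay and manages the boss health bar shown during combat.
; Activate_Boss_Combat creates the health bar widget and adds it to the viewport, while Deactivate_Boss_Combat removes it and clears the reference.
; While the widget is valid, Tick updates its bar each frame from the ratio of Health to MaxHealth.
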(event Custom|Activate_Boss_Combat
  (bind _returnvalue (UserInterface|CreateWidget "/Game/UI/WB_Boss_Health_Bar.WB_Boss_Health_Bar_C"))
  (bind _output_get (Variables|Default|Setboss_health_bar_widget _returnvalue))
  (UserInterface|Viewport|AddtoViewport _output_get 0))

(event Custom|Deactivate_Boss_Combat
  (Widget|RemovefromParent (Variables|Default|Getboss_health_bar_widget))
  (Variables|Default|Setboss_health_bar_widget 0))

(event EventBeginPlay
  (AI|RunBehaviorTree "/Game/AI/Boss/BT_AI_Boss.BT_AI_Boss"))

(event EventTick
  (params (DeltaSeconds :type Float%20%28single-precision%29))
  (bind _boss_health_bar_widget (Variables|Default|Getboss_health_bar_widget)
    (:then
      (Progress|SetPercent (Variables|/Game/UI/WB_Boss_Health_Bar.WB_Boss_Health_Bar_C|GetHealth_Bar _boss_health_bar_widget) (/ (Variables|Default|Gethealth) (Variables|Default|Getmax_health))))
    (:else)))

(fn ConstructionScript
  (|CallParentFunction))