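; BP_Patrol_Route is a spline-based patrol path for the Smart AI enemies.
; It exposes the world position of the spline point at the current PatrolIndex.
; Increment_Patrol_Route steps the index by Direction and flips Direction at the last and first points, so the route runs back and forth instead of looping.
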(event Custom|Increment_Patrol_Route
  (bind _output_get (Variables|Default|Setpatrol_index (+ (Variables|Default|Getpatrol_index) (Variables|Default|Getdirection))))
  (if (== _output_get (- (Spline|GetNumberOfSplinePoints (Variables|Default|GetPatrol%20Route)) 1))
    (Variables|Default|Setdirection -1)
    (elif (== (Variables|Default|Getpatrol_index) 0)
      (Variables|Default|Setdirection 1))))

(fn ConstructionScript)

(fn GetSplinePointasWorldPosition
  (return (Spline|GetLocationatSplinePoint (Variables|Default|GetPatrol%20Route) (Variables|Default|Getpatrol_index) "World")))