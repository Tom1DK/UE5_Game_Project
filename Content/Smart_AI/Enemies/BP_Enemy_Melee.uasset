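; Melee enemy Blueprint that adds a sword attack and montage-driven weapon equip and unequip to its parent class.
; Attack blocks interruption through the combat component during its montage, and a notify sphere-traces forward for pawns to send damage.
; Equip and unequip montage notifies spawn and attach the sword to the hand socket, or destroy it.
; Montage endings fire parent dispatchers, though equip calls OnWeaponUnequipped and unequip calls OnWeaponEquipped.
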(event EventEquipWeapon
  (bind _notifyname (Animation|Montage|PlayMontage (Variables|Character|GetMesh) "/Game/Characters/RPG_Character/Animations_Mix/Animations/Sword/Unsheath_Sword_Montage.Unsheath_Sword_Montage")
    (:OnCompleted
      (Default|CallOnWeaponUnequipped))
    (:OnNotifyBegin
      (switch name _notifyname
        (:Hold%20Sword
          (bind _returnvalue (Game|SpawnActorfromClass "/Game/Weapons/Sword/BP_Weapon_Sword.BP_Weapon_Sword_C" (Transformation|GetActorTransform) "Undefined" "MultiplyWithRoot" 0 0))
          (bind _output_get (Variables|Default|Setweapon_actor _returnvalue))
          (Transformation|AttachComponentToComponent _output_get (Variables|Character|GetMesh) "hand_r_weapon" "SnapToTarget" "SnapToTarget" "SnapToTarget" true)
          (Variables|Default|Setis_wielding_weapon true))))))

(event EventUnequipWeapon
  (bind _notifyname (Animation|Montage|PlayMontage (Variables|Character|GetMesh) "/Game/Characters/RPG_Character/Animations_Mix/Animations/Sword/Sheath_Sword_Montage.Sheath_Sword_Montage")
    (:OnCompleted
      (Default|CallOnWeaponEquipped))
    (:OnNotifyBegin
      (switch name _notifyname
        (:Drop%20Sword
          (Actor|DestroyActor (Variables|Default|Getweapon_actor))
          (Variables|Default|Setis_wielding_weapon false))))))

(event EventAttack
  (bind _returnvalue (Transformation|GetActorLocation))
  (bind _notifyname (Animation|Montage|PlayMontage (Variables|Character|GetMesh) "/Game/Characters/RPG_Character/Animations/Sword_Attacks/Attack1_Montage_Smart_AI.Attack1_Montage_Smart_AI")
    (:then
      (Variables|/Game/Combat_System/BPC_Combat_System.BPC_Combat_System_C|Setis_interruptable (Variables|Default|GetBPC_Combat_System) false))
    (:OnCompleted
      (Default|CallOnAttackEnd :!label _label)
      (Variables|/Game/Combat_System/BPC_Combat_System.BPC_Combat_System_C|Setis_interruptable (Variables|Default|GetBPC_Combat_System) true))
    (:OnInterrupted
      (goto _label))
    (:OnNotifyBegin
      (switch name _notifyname
        (:Slash
          (bind (_outhit _returnvalue_2) (Collision|SphereTraceForObjects _returnvalue (+ _returnvalue (* (Transformation|GetActorForwardVector) 2e+02)) 25.0 (Utilities|Array|MakeArray "ObjectTypeQuery3") false 0 "ForDuration" true "(R=1.000000,G=0.000000,B=0.000000,A=1.000000)" "(R=0.000000,G=1.000000,B=0.000000,A=1.000000)" 2.0))
          (if _returnvalue_2
            (Class|BPIDamagable|TakeDamage(Message) (.HitActor (Collision|BreakHitResult _outhit)) (Utilities|Struct|MakeS_Damage_Info 12.0 "NewEnumerator1"))))))))

(event EventBeginPlay
  (|CallParentFunction))

(fn ConstructionScript
  (|CallParentFunction))