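; Mage enemy Blueprint with a ranged fireball attack and a teleport, plus overrides for movement speed, ideal range and team.
; Attack plays a montage whose Release notify fires a fireball from the right hand through the attack system component.
; Teleport fakes a blink by hiding the mesh, ignoring pawn collision and flying quickly via AI MoveTo with particle trails, then restoring walking.
; Attack token reservation always returns false.
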(event Custom|Teleport
  (params (location :type Vector))
  (bind _charactermovement (Variables|Character|GetCharacterMovement))
  (bind _mesh (Variables|Character|GetMesh))
  (if (not (Variables|Default|Getis_teleporting))
    (Variables|Default|Setis_teleporting true)
    (Pawn|Components|CharacterMovement|SetMovementMode _charactermovement "MOVE_Flying" 0)
    (Variables|/Script/Engine.CharacterMovementComponent|SetMaxFlySpeed _charactermovement 2.5e+03)
    (Variables|/Script/Engine.CharacterMovementComponent|SetMaxAcceleration _charactermovement 2.5e+03)
    (Rendering|SetVisibility _mesh false true)
    (Collision|SetCollisionResponsetoChannel (Variables|Default|GetCapsuleComponent) "ECC_Pawn" "ECR_Ignore")
    (bind _returnvalue (Effects|SpawnEmitterAttached "/Game/VFX/Spells/Shadow_Magic/Particles/Gideon/Abilities/Burden/FX/P_Gideon_Burden_DoT.P_Gideon_Burden_DoT" _mesh "Spine1"))
    (Variables|Default|Setmage_effect_teleport_start _returnvalue)
    (bind _returnvalue_2 (Effects|SpawnEmitterAttached "/Game/VFX/Spells/Shadow_Magic/Particles/Gideon/Abilities/Meteor/FX/P_Gideon_Meteor_Trail.P_Gideon_Meteor_Trail" _mesh "Spine1"))
    (Variables|Default|Setmage_effect_teleport_end _returnvalue_2)
    (Animation|StopAnimMontage 0)
    (AI|AIMoveTo self location 0 2.5e+02 false
      (:OnSuccess
        _)
      (:OnFail
        _))
    (CallFunction|TeleportEnd)
    (else
      (Utilities|FlowControl|DelayUntilNextTick)
      (Default|CallOnTeleportEnd))))

(event Custom|Teleport_End
  (bind _charactermovement (Variables|Character|GetCharacterMovement))
  (Components|Movement|StopMovementImmediately _charactermovement)
  (Pawn|Components|CharacterMovement|SetMovementMode _charactermovement "MOVE_Walking" 0)
  (Variables|/Script/Engine.CharacterMovementComponent|SetMaxAcceleration _charactermovement 1.5e+03)
  (Rendering|SetVisibility (Variables|Character|GetMesh) true true)
  (Collision|SetCollisionResponsetoChannel (Variables|Default|GetCapsuleComponent) "ECC_Pawn" "ECR_Block")
  (Default|CallOnTeleportEnd)
  (Utilities|FlowControl|Delay 0.5)
  (Variables|Default|Setis_teleporting false)
  (Utilities|FlowControl|Sequence
    (:then_0
      (bind _mage_effect_teleport_start (Variables|Default|Getmage_effect_teleport_start)
        (:then
          (Components|DestroyComponent _mage_effect_teleport_start))
        (:else)))
    (:then_1
      (bind _mage_effect_teleport_end (Variables|Default|Getmage_effect_teleport_end)
        (:then
          (Components|DestroyComponent _mage_effect_teleport_end))
        (:else)))))

(event EventAttack
  (params (attack_target :type Actor%20Object%20Reference))
  (|CallParentFunction 0)
  (bind _notifyname (Animation|Montage|PlayMontage (Variables|Character|GetMesh) "/Game/Characters/Mage/Animations/Mage_Fireball_Montage.Mage_Fireball_Montage")
    (:OnCompleted
      (CallFunction|AttackEnd :!label _label))
    (:OnInterrupted
      (goto _label))
    (:OnNotifyBegin
      (switch name _notifyname
        (:Release
          (Default|Fireball (Variables|Default|GetBPC_Attack_System) (Math|Transform|MakeTransform (Transformation|GetSocketLocation (Variables|Character|GetMesh) "RightHand") "0, 0, 0" "1.000000,1.000000,1.000000") attack_target (Utilities|Struct|MakeS_Damage_Info 5.0 "NewEnumerator2" "NewEnumerator1")))))))

(fn ConstructionScript
  (|CallParentFunction))

(fn SetMovementSpeed
  (params (Speed :type E_Movement_Speed%20Enum :default "NewEnumerator0"))
  (return (Utilities|Select :Index Speed :NewEnumerator0 0.0 :NewEnumerator1 125.0 :NewEnumerator2 2.5e+02 :NewEnumerator3 4.2e+02)))

(fn GetIdealRange
  (return 1.2e+03 2.4e+03))

(fn GetTeamNumber
  (return (Variables|Default|Getteam_number)))

(fn ReserveAttackToken
  (params (amount :type Integer))
  (return false))