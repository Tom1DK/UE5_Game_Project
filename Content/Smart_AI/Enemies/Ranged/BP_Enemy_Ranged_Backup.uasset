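; Ranged enemy Blueprint, apparently a backup, that fights with a bow on top of a parent enemy class.
; On BeginPlay it spawns a bow, attaches it to the left-hand socket and signals that a weapon is equipped.
; Attack plays a bow montage whose notify has the attack system component shoot a blockable arrow from the weapon toward the target.
; Overrides supply movement speeds and ideal attack and defend ranges.
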(event EventBeginPlay
  (|CallParentFunction)
  (CallFunction|EquipWeapon))

(event EventEquipWeapon
  ;[1 1 1 1 62] Equip Weapons
  (bind _returnvalue (Game|SpawnActorfromClass "/Game/Weapons/Sword/BP_Weapon_Bow.BP_Weapon_Bow_C" (Math|Transform|MakeTransform "0, 0, 0") "Undefined" "MultiplyWithRoot" 0 0))
  (bind _output_get (Variables|Default|Setweapon_actor _returnvalue))
  (Transformation|AttachComponentToComponent _output_get (Variables|Character|GetMesh) "hand_l_weapon" "SnapToTarget" "SnapToTarget" "SnapToTarget" true)
  (Variables|Default|Setis_wielding_weapon true)
  (Default|CallOnWeaponEquipped))

(event EventAttack
  (params (attack_target :type Actor%20Object%20Reference))
  ;[1 1 1 1 62] Ranged Attack
  (|CallParentFunction attack_target)
  (bind _notifyname (Animation|Montage|PlayMontage (Variables|Character|GetMesh) "/Game/Characters/RPG_Character/Animations_Mix/Animations/Bow/Montage/Bow_Ready_Arrow_Montage1.Bow_Ready_Arrow_Montage1")
    (:OnCompleted
      (CallFunction|AttackEnd attack_target :!label _label))
    (:OnInterrupted
      (goto _label))
    (:OnNotifyBegin
      (switch name _notifyname
        (:Fire
          (Default|ShootArrow (Variables|Default|GetBPC_Attack_System) (Transformation|GetActorLocation (Variables|Default|Getweapon_actor)) (Transformation|GetActorLocation attack_target) (Utilities|Struct|MakeS_Damage_Info 6.0 "NewEnumerator2" "NewEnumerator1" true)))))))

(fn ConstructionScript
  (|CallParentFunction))

(fn SetMovementSpeed
  (params (Speed :type E_Movement_Speed%20Enum :default "NewEnumerator0"))
  (bind _output_get (Variables|/Script/Engine.CharacterMovementComponent|SetMaxWalkSpeed (Variables|Character|GetCharacterMovement) (Utilities|Select :Index Speed :NewEnumerator0 0.0 :NewEnumerator1 2e+02 :NewEnumerator2 3e+02 :NewEnumerator3 4.1e+02)))
  (return _output_get))

(fn GetIdealRange
  (return 8e+02 8e+02))