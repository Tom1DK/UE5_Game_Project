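; Melee enemy Blueprint that fights with sword and shield, extending a parent enemy class.
; Montage notifies spawn and attach weapons, destroy the referenced weapon on sheathing, and trigger a forward sphere-trace hit during uninterruptible attacks.
; Blockable damage randomly starts a timed block through the combat component before damage is applied; a successful block plays a shield reaction, then ends blocking.
; Equip and unequip completions fire each other's dispatchers, and the block-idle montage is disconnected.
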(event OnBlocked(BPC_Combat_System)
  (params (can_be_parried :type Boolean))
  ;[1 1 1 1 62] Block System
  (Variables|Default|Setblocking_state "NewEnumerator2")
  (Utilities|Time|ClearandInvalidateTimerbyHandle (Variables|Default|Gethold_block_time))
  (Animation|Montage|PlayMontage (Variables|Character|GetMesh) "/Game/Characters/RPG_Character/Animations_Mix/Animations/Sword/Montage/Shield_Block_React_Montage.Shield_Block_React_Montage"
    (:OnCompleted
      _)
    (:OnInterrupted
      _))
  (CallFunction|EndBlock))

(event Custom|Start_Block
  ;[1 1 1 1 62] Block System
  (Utilities|Time|ClearandInvalidateTimerbyHandle (Variables|Default|Gethold_block_time))
  (Components|Movement|StopMovementImmediately (Variables|Character|GetCharacterMovement))
  (Variables|/Game/Combat_System/BPC_Combat_System.BPC_Combat_System_C|Setis_blocking (Variables|Default|GetBPC_Combat_System) true)
  (Variables|Default|Setblocking_state "NewEnumerator1")
  (Components|Movement|StopMovementImmediately (Variables|Character|GetCharacterMovement))
  (bind _returnvalue (Utilities|Time|SetTimerbyEvent (EventDispatchers|CreateEvent :!event Custom|End_Block) 2.0))
  (Variables|Default|Sethold_block_time _returnvalue))

(event Custom|End_Block
  ;[1 1 1 1 62] Block System
  (Variables|/Game/Combat_System/BPC_Combat_System.BPC_Combat_System_C|Setis_blocking (Variables|Default|GetBPC_Combat_System) false)
  (Variables|Default|Setblocking_state "NewEnumerator0")
  (Default|CallOnBlockEnded))

(event EventEquipWeapon
  (bind _returnvalue (Transformation|GetActorTransform))
  (bind _mesh (Variables|Character|GetMesh))
  ;[1 1 1 1 62] Equip Weapons
  (bind _notifyname (Animation|Montage|PlayMontage (Variables|Character|GetMesh) "/Game/Characters/RPG_Character/Animations_Mix/Animations/Sword/Montage/Unsheath_Sword_Montage.Unsheath_Sword_Montage")
    (:OnCompleted
      (Default|CallOnWeaponUnequipped))
    (:OnNotifyBegin
      (switch name _notifyname
        (:Hold%20Sword
          (bind _returnvalue_2 (Game|SpawnActorfromClass "/Game/Weapons/Sword/BP_Weapon_Sword.BP_Weapon_Sword_C" _returnvalue "Undefined" "MultiplyWithRoot" 0 0))
          (bind _output_get (Variables|Default|Setweapon_actor _returnvalue_2))
          (Transformation|AttachComponentToComponent _output_get _mesh "hand_r_weapon" "SnapToTarget" "SnapToTarget" "SnapToTarget" true))
        (:Hold%20Shield
          (bind _returnvalue_3 (Game|SpawnActorfromClass "/Game/Weapons/Sword/BP_Weapon_Shield.BP_Weapon_Shield_C" _returnvalue "Undefined" "MultiplyWithRoot" 0 0))
          (bind _output_get_2 (Variables|Default|Setweapon_actor _returnvalue_3))
          (Transformation|AttachComponentToComponent _output_get_2 _mesh "hand_l_off_hand" "SnapToTarget" "SnapToTarget" "SnapToTarget" true)))
      (Variables|Default|Setis_wielding_weapon true))))

(event EventUnequipWeapon
  ;[1 1 1 1 62] Equip Weapons
  (bind _notifyname (Animation|Montage|PlayMontage (Variables|Character|GetMesh) "/Game/Characters/RPG_Character/Animations_Mix/Animations/Sword/Montage/Sheath_Sword_Montage.Sheath_Sword_Montage")
    (:OnCompleted
      (Default|CallOnWeaponEquipped))
    (:OnNotifyBegin
      (switch name _notifyname
        (:Drop%20Sword
          (Actor|DestroyActor (Variables|Default|Getweapon_actor))
          (Variables|Default|Setis_wielding_weapon false))))))

(event EventAttack
  (params (attack_target :type Actor%20Object%20Reference))
  (bind _returnvalue (Transformation|GetActorLocation))
  ;[1 1 1 1 62] Attack
  (|CallParentFunction attack_target)
  (bind _notifyname (Animation|Montage|PlayMontage (Variables|Character|GetMesh) "/Game/Characters/RPG_Character/Animations_Mix/Animations/Sword/Montage/Weapon_Attack_Sword_and_Shield_Montage.Weapon_Attack_Sword_and_Shield_Montage")
    (:then
      (Variables|/Game/Combat_System/BPC_Combat_System.BPC_Combat_System_C|Setis_interruptable (Variables|Default|GetBPC_Combat_System) false))
    (:OnCompleted
      (CallFunction|AttackEnd attack_target :!label _label)
      (Variables|/Game/Combat_System/BPC_Combat_System.BPC_Combat_System_C|Setis_interruptable (Variables|Default|GetBPC_Combat_System) true))
    (:OnInterrupted
      (goto _label))
    (:OnNotifyBegin
      (switch name _notifyname
        (:Slash
          (bind (_outhit _returnvalue_2) (Collision|SphereTraceForObjects _returnvalue (+ _returnvalue (* 2e+02 (Transformation|GetActorForwardVector))) 25.0 (Utilities|Array|MakeArray "ObjectTypeQuery3") false 0 "ForDuration" true "(R=1.000000,G=0.000000,B=0.000000,A=1.000000)" "(R=0.000000,G=1.000000,B=0.000000,A=1.000000)" 2.0))
          (if _returnvalue_2
            (Class|BPIDamagable|TakeDamage(Message) (.HitActor (Collision|BreakHitResult _outhit)) (Utilities|Struct|MakeS_Damage_Info 1.0 "NewEnumerator1") self)))))))

(event EventBeginPlay
  (|CallParentFunction))

(fn ConstructionScript
  (|CallParentFunction))

(fn TakeDamage
  (params (damage_info :type S%20Damage%20Info%20Structure) (damage%20causer :type Actor%20Object%20Reference))
  (if (.Is_Blockable (Utilities|Struct|BreakS_Damage_Info damage_info))
    (CallFunction|TrytoBlock))
  (bind _was_damaged (Default|TakeDamage (Variables|Default|GetBPC_Combat_System) damage_info damage%20causer))
  (return _was_damaged))

(fn TrytoBlock
  (if (<= (Math|Random|RandomFloat) (Variables|Default|Getblock_chance))
    (CallFunction|StartBlock)))