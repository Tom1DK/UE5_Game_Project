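; Base enemy character that exposes damage, healing, team, patrol, range and speed functions, delegating health and combat to BPCCombatSystem.
; Combat component events drive AIC_Enemy_Base states: hits play a stagger montage, then attack the causer with temporary uninterruptibility, while death ragdolls and stops AI logic.
; Attacks reserve tokens from the target, tracked per target and returned on attack end or death.
; Also adds a health bar widget and arc-launched jumps.
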(event Custom|Death
  (bind _mesh (Variables|Character|GetMesh))
  ;[1 1 1] Death
  (Physics|SetSimulatePhysics _mesh true)
  (Collision|SetCollisionEnabled _mesh "QueryAndPhysics")
  (AI|Logic|StopLogic (Variables|/Script/AIModule.AIController|GetBrainComponent (Variables|Default|Getaic_enemy_base)) "")
  (Default|SetStateasDead (Variables|Default|Getaic_enemy_base))
  (bind _keys (Utilities|Map|Keys (Variables|Default|Getreserved_attack_tokens)))
  (for _array_element _keys
    (Class|BPIDamagable|ReturnAttackToken(Message) _array_element (.Value (Utilities|Map|Find (Variables|Default|Getreserved_attack_tokens) _array_element)))))

(event Custom|Hit_Response
  (params (damage_response :type E_Damage_Response%20Enum :default "NewEnumerator0") (damage_causer :type Actor%20Object%20Reference))
  ;[1 1 1] Hit Response
  (Components|Movement|StopMovementImmediately (Variables|Character|GetCharacterMovement))
  (Default|SetStateasStaggered (Variables|Default|Getaic_enemy_base))
  (Animation|Montage|PlayMontage (Variables|Character|GetMesh) (Variables|Default|Gethit_reaction_montage) 1.5
    (:OnCompleted
      _)
    (:OnInterrupted
      _))
  (Default|SetStateasAttacking (Variables|Default|Getaic_enemy_base) damage_causer true)
  (Variables|/Game/Combat_System/BPC_Combat_System.BPC_Combat_System_C|Setis_interruptable (Variables|Default|GetBPC_Combat_System) false)
  (Utilities|FlowControl|Delay 5.0)
  (Variables|/Game/Combat_System/BPC_Combat_System.BPC_Combat_System_C|Setis_interruptable (Variables|Default|GetBPC_Combat_System) true))

(event EventJumptoDestination
  (params (destination :type Vector :default "0, 0, 0"))
  (bind (_x _y _z) (Math|Vector|BreakVector destination))
  ;[1 1 1] Enemy Jump
  (bind _outlaunchvelocity (Game|SuggestProjectileVelocityCustomArc (Transformation|GetActorLocation) (Math|Vector|MakeVector _x _y (+ _z 2.5e+02)) 0.0 0.5))
  (Character|LaunchCharacter _outlaunchvelocity true true))

(event EventBeginPlay
  (bind _bpc_combat_system (Variables|Default|GetBPC_Combat_System))
  (bind _asaic_enemy_base (Utilities|Casting|CastToAIC_Enemy_Base (AI|GetAIController self)))
  (Variables|Default|Setaic_enemy_base _asaic_enemy_base)
  (bind _returnvalue (UserInterface|CreateWidget "/Game/UI/WB_New_Health_Bar.WB_New_Health_Bar_C" 0 self))
  (UserInterface|SetWidget (Variables|Default|GetHealth%20Bar) _returnvalue)
  (EventDispatchers|BindEventtoOnDeath _bpc_combat_system (EventDispatchers|CreateEvent :!event Custom|Death))
  (EventDispatchers|BindEventtoOnDamageResponse _bpc_combat_system (EventDispatchers|CreateEvent :!event Custom|Hit_Response)))

(event EventReturnAttackToken
  (params (amount :type Integer))
  (Default|ReturnAttackToken (Variables|Default|GetBPC_Combat_System) amount))

(event EventStoreAttackTokens
  (params (attack_target :type Actor%20Object%20Reference) (amount_of_tokens_stored :type Integer))
  (bind _reserved_attack_tokens (Variables|Default|Getreserved_attack_tokens))
  (bind (_value _returnvalue) (Utilities|Map|Find _reserved_attack_tokens attack_target))
  (Utilities|Map|Add (Variables|Default|Getreserved_attack_tokens) attack_target (Math|Integer|SelectInt (+ amount_of_tokens_stored _value) amount_of_tokens_stored _returnvalue)))

(event EventAttackEnd
  (params (attack_target :type Actor%20Object%20Reference))
  (bind _tokens_used_in_current_attack (Variables|Default|Gettokens_used_in_current_attack))
  (Class|BPIDamagable|ReturnAttackToken(Message) attack_target _tokens_used_in_current_attack)
  (CallFunction|StoreAttackTokens attack_target (* _tokens_used_in_current_attack -1))
  (Variables|Default|Setattacking false)
  (Default|CallOnAttackEnd))

(event EventAttack
  (params (attack_target :type Actor%20Object%20Reference))
  (Variables|Default|Setattacking true))

(fn ConstructionScript
  (bind _bpc_combat_system (Variables|Default|GetBPC_Combat_System))
  (Variables|/Game/Combat_System/BPC_Combat_System.BPC_Combat_System_C|Setmax_health _bpc_combat_system (Variables|/Game/Combat_System/BPC_Combat_System.BPC_Combat_System_C|Getmax_health _bpc_combat_system))
  (Variables|/Game/Combat_System/BPC_Combat_System.BPC_Combat_System_C|Setcurrent_health _bpc_combat_system (Variables|/Game/Combat_System/BPC_Combat_System.BPC_Combat_System_C|Getcurrent_health _bpc_combat_system)))

(fn Vault)

(fn AttatchtoSerfaceCalculation
  (params (Attatch%20Distance :type Float%20%28single-precision%29))
  (bind _returnvalue (Transformation|GetActorLocation))
  (bind (_outhit _returnvalue_2) (Collision|LineTraceByChannel _returnvalue (+ _returnvalue (* (Math|Vector|GetForwardVector (Transformation|GetActorRotation)) Attatch%20Distance)) "TraceTypeQuery1" false 0 "ForDuration"))
  (return _outhit _returnvalue_2))

(fn AttackStart
  (params (attack_target :type Actor%20Object%20Reference) (tokens_needed_to_attack :type Integer))
  (bind _success (Class|BPIDamagable|ReserveAttackToken(Message) attack_target tokens_needed_to_attack))
  (if _success
    (CallFunction|StoreAttackTokens attack_target tokens_needed_to_attack)
    (Variables|Default|Settokens_used_in_current_attack tokens_needed_to_attack)
    (return true)
    (else
      (return false))))

(fn GetCurrentHealth
  (return (Variables|/Game/Combat_System/BPC_Combat_System.BPC_Combat_System_C|Getcurrent_health (Variables|Default|GetBPC_Combat_System))))

(fn GetIdealRange
  (return 1.2e+02 3.5e+02))

(fn GetMaxHealth
  (return (Variables|/Game/Combat_System/BPC_Combat_System.BPC_Combat_System_C|Getmax_health (Variables|Default|GetBPC_Combat_System))))

(fn GetPatrolRoute
  (return (Variables|Smart_AI|Getpatrol_route)))

(fn GetTeamNumber
  (return (Variables|Default|Getteam_number)))

(fn Heal
  (params (ammount_healed :type Float%20%28double-precision%29))
  (bind _new_health (Default|Heal (Variables|Default|GetBPC_Combat_System) ammount_healed))
  (return _new_health))

(fn IsAttacking
  (return (Variables|Default|Getattacking)))

(fn IsDead
  (return (Variables|/Game/Combat_System/BPC_Combat_System.BPC_Combat_System_C|Getis_dead (Variables|Default|GetBPC_Combat_System))))

(fn ReserveAttackToken
  (params (amount :type Integer))
  (bind _success (Default|ReserveAttackToken (Variables|Default|GetBPC_Combat_System) amount))
  (return _success))

(fn SetMovementSpeed
  (params (Speed :type E_Movement_Speed%20Enum :default "NewEnumerator0"))
  (bind _output_get (Variables|/Script/Engine.CharacterMovementComponent|SetMaxWalkSpeed (Variables|Character|GetCharacterMovement) (Utilities|Select :Index Speed :NewEnumerator0 0.0 :NewEnumerator1 125.0 :NewEnumerator2 2.8e+02 :NewEnumerator3 4.1e+02)))
  (return _output_get))

(fn TakeDamage
  (params (damage_info :type S%20Damage%20Info%20Structure) (damage%20causer :type Actor%20Object%20Reference))
  (bind _was_damaged (Default|TakeDamage (Variables|Default|GetBPC_Combat_System) damage_info damage%20causer))
  (return _was_damaged))