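; Melee enemy child Blueprint that fights with sword and shield, equipped and sheathed through montage notifies.
; Attack currently runs a jump slash that launches toward the target's predicted position; short-range and spinning chase-plus-AOE attacks are also defined.
; Montage notifies drive sphere-trace damage, movement and AOE spawning.
; Blockable hits randomly trigger a timed shield block before damage passes to BPC Combat System, whose OnBlocked event plays the reaction.
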(event OnBlocked(BPC_Combat_System)
  (params (can_be_parried :type Boolean))
  ;[1 1 1 1 62] Block System
  (Variables|Default|Setblocking_state "NewEnumerator2")
  (Utilities|Time|ClearandInvalidateTimerbyHandle (Variables|Default|Gethold_block_time))
  (Animation|Montage|PlayMontage (Variables|Character|GetMesh) "/Game/Characters/RPG_Character/Animations_Mix/Animations/Sword/Montage/Shield_Block_React_Montage.Shield_Block_React_Montage"
    (:OnCompleted
      _)
    (:OnInterrupted
      _))
  (CallFunction|EndBlock))

(event Custom|Spinning_Attack
  (params (attack_target :type Actor%20Object%20Reference))
  ;[1 1 1 1 62] Attack
  (|CallParentFunction attack_target)
  (bind _notifyname (Animation|Montage|PlayMontage (Variables|Character|GetMesh) "/Game/Characters/RPG_Character/Animations/Sword_Attacks/Montages/Sword_Spin_Attack_Montage.Sword_Spin_Attack_Montage")
    (:then
      (Variables|/Game/Combat_System/BPC_Combat_System.BPC_Combat_System_C|Setis_interruptable (Variables|Default|GetBPC_Combat_System) true))
    (:OnCompleted
      (CallFunction|AttackEnd attack_target :!label _label)
      (Variables|/Game/Combat_System/BPC_Combat_System.BPC_Combat_System_C|Setis_interruptable (Variables|Default|GetBPC_Combat_System) true))
    (:OnInterrupted
      (goto _label))
    (:OnNotifyBegin
      (switch name _notifyname
        (:Slash
          (CallFunction|SphereTraceDamage)
          (CallFunction|StopSpinning))
        (:Spin
          (CallFunction|SpinMesh)
          (CallFunction|ChaseAttackTarget attack_target))
        (:AOE_Slash
          (CallFunction|AOESlash attack_target))))))

(event Custom|Long_Range_Attack
  (params (attack_target :type Actor%20Object%20Reference))
  ;[1 1 1 1 62] Attack
  (|CallParentFunction attack_target)
  (bind _notifyname (Animation|Montage|PlayMontage (Variables|Character|GetMesh) "/Game/Characters/RPG_Character/Animations/Sword_Attacks/Montages/Sword_Jump_Attack_Montage.Sword_Jump_Attack_Montage")
    (:then
      (Variables|/Game/Combat_System/BPC_Combat_System.BPC_Combat_System_C|Setis_interruptable (Variables|Default|GetBPC_Combat_System) false))
    (:OnCompleted
      (CallFunction|AttackEnd attack_target :!label _label)
      (Variables|/Game/Combat_System/BPC_Combat_System.BPC_Combat_System_C|Setis_interruptable (Variables|Default|GetBPC_Combat_System) true))
    (:OnInterrupted
      (goto _label))
    (:OnNotifyBegin
      (switch name _notifyname
        (:Slash
          (CallFunction|SphereTraceDamage))
        (:Jump
          (CallFunction|JumptoAttackTarget attack_target)
          (Default|TakeDamage (Variables|Default|GetBPC_Combat_System)))))))

(event Custom|Stop_Spinning
  ;[1 1 1 1 62] Attack
  (Audio|Components|Audio|Stop (Variables|Default|GetSpin_Mesh_Timeline))
  (Transformation|SetRelativeRotation (Variables|Character|GetMesh) (Variables|Default|Getmesh_rotation_before_spin) false false))

(event Custom|AOE_Slash
  (params (attack_target :type Actor%20Object%20Reference))
  ;[1 1 1 1 62] Attack
  (bind _returnvalue (Game|SpawnActorfromClass "/Game/Combat_System/AOE/BP_Base_AOE.BP_Base_AOE_C" (Math|Transform|MakeTransform (Transformation|GetActorLocation) "0, 0, 0" "1.000000,1.000000,1.000000") "Undefined" "MultiplyWithRoot" 0 3e+02 true true false self))
  (EventDispatchers|BindEventtoOnAOEOverlapActor _returnvalue (delegate Custom|CustomEvent))
  (Default|Trigger _returnvalue))

(event Custom|CustomEvent
  (params (actor :type Actor%20Object%20Reference))
  ;[1 1 1 1 62] Attack
  (if (== actor (stale Custom|AOE_Slash attack_target))
    (Class|BPIDamagable|TakeDamage(Message) actor (Utilities|Struct|MakeS_Damage_Info 4.0 "NewEnumerator1" "NewEnumerator1") self)))

(event Custom|Sphere_Trace_Damage
  (bind _returnvalue (Transformation|GetActorLocation))
  ;[1 1 1 1 62] Attack Helper
  (bind (_outhit _returnvalue_2) (Collision|SphereTraceForObjects _returnvalue (+ _returnvalue (* 2e+02 (Transformation|GetActorForwardVector))) 25.0 (Utilities|Array|MakeArray "ObjectTypeQuery3") false 0 "ForDuration" true "(R=1.000000,G=0.000000,B=0.000000,A=1.000000)" "(R=0.000000,G=1.000000,B=0.000000,A=1.000000)" 2.0))
  (if _returnvalue_2
    (Class|BPIDamagable|TakeDamage(Message) (.HitActor (Collision|BreakHitResult _outhit)) (Utilities|Struct|MakeS_Damage_Info 1.0 "NewEnumerator1") self)))

(event Custom|Start_Block
  ;[1 1 1 1 62] Block System
  (Utilities|Time|ClearandInvalidateTimerbyHandle (Variables|Default|Gethold_block_time))
  (Components|Movement|StopMovementImmediately (Variables|Character|GetCharacterMovement))
  (Variables|/Game/Combat_System/BPC_Combat_System.BPC_Combat_System_C|Setis_blocking (Variables|Default|GetBPC_Combat_System) true)
  (Variables|Default|Setblocking_state "NewEnumerator1")
  (Components|Movement|StopMovementImmediately (Variables|Character|GetCharacterMovement))
  (bind _returnvalue (Utilities|Time|SetTimerbyEvent (EventDispatchers|CreateEvent :!event Custom|End_Block) 2.0))
  (Variables|Default|Sethold_block_time _returnvalue))

(event Custom|Short_Range_Attack
  (params (attack_target :type Actor%20Object%20Reference))
  ;[1 1 1 1 62] Attack
  (|CallParentFunction 0)
  (bind _notifyname (Animation|Montage|PlayMontage (Variables|Character|GetMesh) "/Game/Characters/RPG_Character/Animations_Mix/Animations/Sword/Montage/Weapon_Attack_Sword_and_Shield_Montage.Weapon_Attack_Sword_and_Shield_Montage")
    (:then
      (Variables|/Game/Combat_System/BPC_Combat_System.BPC_Combat_System_C|Setis_interruptable (Variables|Default|GetBPC_Combat_System) false))
    (:OnCompleted
      (CallFunction|AttackEnd attack_target :!label _label)
      (Variables|/Game/Combat_System/BPC_Combat_System.BPC_Combat_System_C|Setis_interruptable (Variables|Default|GetBPC_Combat_System) true))
    (:OnInterrupted
      (goto _label))
    (:OnNotifyBegin
      (switch name _notifyname
        (:Slash
          (CallFunction|SphereTraceDamage))))))

(event Custom|End_Block
  ;[1 1 1 1 62] Block System
  (Variables|/Game/Combat_System/BPC_Combat_System.BPC_Combat_System_C|Setis_blocking (Variables|Default|GetBPC_Combat_System) false)
  (Variables|Default|Setblocking_state "NewEnumerator0")
  (Default|CallOnBlockEnded))

(event Custom|Spin_Mesh
  (Variables|Default|Setmesh_rotation_before_spin (Variables|/Script/Engine.SceneComponent|GetRelativeRotation (Variables|Character|GetMesh)))
  (bind _z_rotation_alpha (Timeline|Spin_Mesh_Timeline PlayFromStart)
    (:Update
      (Transformation|SetRelativeRotation (Variables|Character|GetMesh) (Math|Rotator|MakeRotator (.roll (Variables|Default|Getmesh_rotation_before_spin)) (.pitch (Variables|Default|Getmesh_rotation_before_spin)) (Math|Float|Lerp (.yaw (Variables|Default|Getmesh_rotation_before_spin)) (+ (.yaw (Variables|Default|Getmesh_rotation_before_spin)) (|(360*10))) _z_rotation_alpha)) false false))))

(event Custom|Jump_to_Attack_Target
  (params (attack_target :type Actor%20Object%20Reference))
  (bind _location (CallFunction|CalculateFutureActorLocation attack_target 1.0))
  (bind _outlaunchvelocity (Game|SuggestProjectileVelocityCustomArc (Transformation|GetActorLocation) (Math|Vector|MakeVector (.x _location) (.y _location) (+ (.z _location) 1e+02)) 0.0 0.5))
  (Character|LaunchCharacter _outlaunchvelocity true true)
  (EventDispatchers|AssignLandedDelegate (delegate Custom|On_Land)))

(event Custom|On_Land
  (params (Hit :type Hit%20Result%20Structure%20%28by%20ref%29))
  (EventDispatchers|UnbindEventfromLandedDelegate (delegate Custom|On_Land))
  (Components|Movement|StopMovementImmediately (Variables|Character|GetCharacterMovement)))

(event Custom|Chase_Attack_Target
  (params (attack_target :type Actor%20Object%20Reference))
  (AI|AIMoveTo self "0, 0, 0" attack_target 2e+02 false
    (:OnSuccess
      (Utilities|FlowControl|Delay 0.1)
      (if (Variables|Default|Getattacking)
        (CallFunction|ChaseAttackTarget attack_target)))))

(event EventEquipWeapon
  (bind _returnvalue (Transformation|GetActorTransform))
  (bind _mesh (Variables|Character|GetMesh))
  ;[1 1 1 1 62] Equip Weapons
  (bind _notifyname (Animation|Montage|PlayMontage (Variables|Character|GetMesh) "/Game/Characters/RPG_Character/Animations_Mix/Animations/Sword/Montage/Unsheath_Sword_Montage.Unsheath_Sword_Montage")
    (:OnCompleted
      (Default|CallOnWeaponUnequipped))
    (:OnNotifyBegin
      (switch name _notifyname
        (:Hold%20Sword
          (bind _returnvalue_2 (Game|SpawnActorfromClass "/Game/Weapons/Sword/BP_Weapon_Sword.BP_Weapon_Sword_C" _returnvalue "Undefined" "MultiplyWithRoot" 0 0))
          (bind _output_get (Variables|Default|Setweapon_actor _returnvalue_2))
          (Transformation|AttachComponentToComponent _output_get _mesh "hand_r_weapon" "SnapToTarget" "SnapToTarget" "SnapToTarget" true))
        (:Hold%20Shield
          (bind _returnvalue_3 (Game|SpawnActorfromClass "/Game/Weapons/Sword/BP_Weapon_Shield.BP_Weapon_Shield_C" _returnvalue "Undefined" "MultiplyWithRoot" 0 0))
          (bind _output_get_2 (Variables|Default|Setweapon_actor _returnvalue_3))
          (Transformation|AttachComponentToComponent _output_get_2 _mesh "hand_l_off_hand" "SnapToTarget" "SnapToTarget" "SnapToTarget" true)))
      (Variables|Default|Setis_wielding_weapon true))))

(event EventUnequipWeapon
  ;[1 1 1 1 62] Equip Weapons
  (bind _notifyname (Animation|Montage|PlayMontage (Variables|Character|GetMesh) "/Game/Characters/RPG_Character/Animations_Mix/Animations/Sword/Montage/Sheath_Sword_Montage.Sheath_Sword_Montage")
    (:OnCompleted
      (Default|CallOnWeaponEquipped))
    (:OnNotifyBegin
      (switch name _notifyname
        (:Drop%20Sword
          (Actor|DestroyActor (Variables|Default|Getweapon_actor))
          (Variables|Default|Setis_wielding_weapon false))))))

(event EventAttack
  (params (attack_target :type Actor%20Object%20Reference))
  ;[1 1 1 1 62] Attack
  (CallFunction|LongRangeAttack attack_target))

(event EventBeginPlay
  (|CallParentFunction))

(fn ConstructionScript
  (|CallParentFunction)
  (Variables|Default|Setmesh_rotation_before_spin (Variables|/Script/Engine.SceneComponent|GetRelativeRotation (Variables|Character|GetMesh))))

(fn TakeDamage
  (params (damage_info :type S%20Damage%20Info%20Structure) (damage%20causer :type Actor%20Object%20Reference))
  (if (.Is_Blockable (Utilities|Struct|BreakS_Damage_Info damage_info))
    (CallFunction|TrytoBlock))
  (bind _was_damaged (Default|TakeDamage (Variables|Default|GetBPC_Combat_System) damage_info damage%20causer))
  (return _was_damaged))

(fn TrytoBlock
  (if (<= (Math|Random|RandomFloat) (Variables|Default|Getblock_chance))
    (CallFunction|StartBlock)))

(fn CalculateFutureActorLocation
  (params (actor :type Actor%20Object%20Reference) (time :type Float%20%28double-precision%29))
  (return (+ (Transformation|GetActorLocation actor) (* time (* (Transformation|GetVelocity actor) "1.000000,1.000000,0.000000")))))

(fn GetIdealRange
  (return 252.0 2.5e+02))