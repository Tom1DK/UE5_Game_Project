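; Target dummy character that takes hits and can be stealth-assassinated from behind.
; Overlapping AssassinationRadius shows an assassinate prompt to the player, billboarded to the camera alongside the health bar.
; Damage plays a random hit montage, launches the dummy along the player's facing and reduces BPCPlayerStats health, ragdolling on death.
; StealthBackAssassination plays the paired victim montage, triggers a delayed ragdoll and returns the attacker's reference location and rotation.
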(event OnComponentBeginOverlap(AssassinationRadius)
  (params (OverlappedComponent :type Primitive%20Component%20Object%20Reference) (OtherActor :type Actor%20Object%20Reference) (OtherComp :type Primitive%20Component%20Object%20Reference) (OtherBodyIndex :type Integer) (bFromSweep :type Boolean) (SweepResult :type Hit%20Result%20Structure%20%28by%20ref%29))
  (Utilities|Casting|CastToBP_ThirdPersonCharacter OtherActor)
  (Rendering|SetVisibility (Variables|Default|GetAssassinate_Widget) true false))

(event OnComponentEndOverlap(AssassinationRadius)
  (params (OverlappedComponent :type Primitive%20Component%20Object%20Reference) (OtherActor :type Actor%20Object%20Reference) (OtherComp :type Primitive%20Component%20Object%20Reference) (OtherBodyIndex :type Integer))
  (Utilities|Casting|CastToBP_ThirdPersonCharacter OtherActor)
  (Rendering|SetVisibility (Variables|Default|GetAssassinate_Widget) false false))

(event Custom|Ragdoll
  ;[1 1 1] Ragdoll
  (Utilities|FlowControl|Sequence
    (:then_0
      (Utilities|FlowControl|Delay 2.5)
      (Physics|SetSimulatePhysics (Variables|Character|GetMesh) true))
    (:then_1
      (Utilities|FlowControl|Delay 2.2)
      (Audio|PlaySoundatLocation "/Game/Audio/Grunts-Hits/SC_Death.SC_Death" (Transformation|GetActorLocation) "0, 0, 0" 1.0 1.0 0.0 "/Game/Audio/UI/SA_Character.SA_Character" 0 0 0))))

(event EventBeginPlay
  (bind _aswb_dummy_healthbar (Utilities|Casting|CastToWB_Dummy_Healthbar (UserInterface|GetWidget (Variables|Default|GetHealth_Bar_Widget))))
  (Variables|Default|Sethealth_bar_ui _aswb_dummy_healthbar))

(event Collision|EventActorBeginOverlap
  (params (OtherActor :type Actor%20Object%20Reference)))

(event EventTick
  (params (DeltaSeconds :type Float%20%28single-precision%29))
  (Transformation|SetWorldRotation (Variables|Default|GetAssassinate_Widget) (Math|Rotator|FindLookatRotation (Transformation|GetWorldLocation (Variables|Default|GetAssassinate_Widget)) (Transformation|GetWorldLocation (Variables|/Script/Engine.PlayerCameraManager|GetTransformComponent (Game|GetPlayerCameraManager 0)))) false false))

(event Game|Damage|EventAnyDamage
  (params (Damage :type Float%20%28single-precision%29) (DamageType :type Damage%20Type%20Object%20Reference) (InstigatedBy :type Controller%20Object%20Reference) (DamageCauser :type Actor%20Object%20Reference))
  (Animation|PlayAnimMontage (Utilities|Array|Get(acopy) (Variables|Default|Gethit_anims) (Math|Random|RandomIntegerinRange 0 (- (Utilities|Array|Length (Variables|Default|Gethit_anims)) 1))) 1.0 "None")
  (bind _asbp_third_person_character (Utilities|Casting|CastToBP_ThirdPersonCharacter (Game|GetPlayerCharacter 0)))
  (Character|LaunchCharacter (* (Math|Vector|GetForwardVector (Transformation|GetActorRotation _asbp_third_person_character)) 7e+02) false false)
  (Audio|PlaySoundatLocation "/Game/Audio/Grunts-Hits/Death2.Death2" (Transformation|GetActorLocation) "0, 0, 0" 1.0 (Math|Random|RandomFloatinRange 0.8 1.0) 0.0 "/Game/Audio/UI/SA_Character.SA_Character" 0 0 0)
  (bind _is_player_dead (Default|DecreaseHealth (Variables|Default|GetBPC_Player_Stats) Damage))
  (if _is_player_dead
    (Physics|SetSimulatePhysics (Variables|Character|GetMesh) true)
    (Audio|PlaySoundatLocation "/Game/Audio/Grunts-Hits/SC_Death.SC_Death" (Transformation|GetActorLocation) "0, 0, 0" 1.0 1.0 0.0 "/Game/Audio/UI/SA_Character.SA_Character" 0 0 0)
    (Rendering|SetVisibility (Variables|Default|GetHealth_Bar_Widget) false false)))

(fn ConstructionScript)

(fn StealthBackAssassination
  (Animation|PlayAnimMontage "/Game/Characters/RPG_Character/Animations/Assassinations/Paired_Knife_Stealth_KidneyAndNeck_Vic_Montage.Paired_Knife_Stealth_KidneyAndNeck_Vic_Montage" 1.0 "None")
  (CallFunction|Ragdoll)
  (Rendering|SetVisibility (Variables|Default|GetAssassinate_Widget) false false)
  (return (Transformation|GetWorldLocation (Variables|Default|GetAssassin_REF)) (Transformation|GetActorRotation)))