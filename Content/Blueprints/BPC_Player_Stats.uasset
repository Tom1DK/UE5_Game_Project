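; Player stats component for BP_ThirdPersonCharacter that tracks health, stamina, XP and level.
; On BeginPlay it waits a tick, caches the owning character and fills its HUD bars and texts.
; Each change function writes straight to that HUD; decreases return whether the stat is depleted, and increases to current health or stamina clamp at max.
; Reaching max XP levels up, raising the XP cap by a fixed step and resetting XP without carrying overflow.
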(event EventBeginPlay
  (Utilities|FlowControl|DelayUntilNextTick)
  (bind _asbp_third_person_character (Utilities|Casting|CastToBP_ThirdPersonCharacter (Components|GetOwner)))
  (Variables|Default|SetPlayer_Character_BP _asbp_third_person_character)
  (Progress|SetPercent (Variables|/Game/UI/WB_HUD.WB_HUD_C|GetStamina_Bar (Variables|/Game/ThirdPerson/Blueprints/BP_ThirdPersonCharacter.BP_ThirdPersonCharacter_C|Gethud_widget (Variables|Default|GetPlayer_Character_BP))) (/ (Variables|Stamina|GetCurrent_Stamina) (Variables|Stamina|GetMax_Stamina)))
  (Progress|SetPercent (Variables|/Game/UI/WB_HUD.WB_HUD_C|GetHealth_Bar (Variables|/Game/ThirdPerson/Blueprints/BP_ThirdPersonCharacter.BP_ThirdPersonCharacter_C|Gethud_widget (Variables|Default|GetPlayer_Character_BP))) (/ (Variables|Health|GetCurrent_Health) (Variables|Health|GetMax_Health)))
  (Rendering|Components|TextRender|SetText (Variables|/Game/UI/WB_HUD.WB_HUD_C|GetHealth_Text (Variables|/Game/ThirdPerson/Blueprints/BP_ThirdPersonCharacter.BP_ThirdPersonCharacter_C|Gethud_widget (Variables|Default|GetPlayer_Character_BP))) (Utilities|Text|ToText(Float) (Variables|Health|GetCurrent_Health) "HalfToEven"))
  (Progress|SetPercent (Variables|/Game/UI/WB_HUD.WB_HUD_C|GetExperienceBar (Variables|/Game/ThirdPerson/Blueprints/BP_ThirdPersonCharacter.BP_ThirdPersonCharacter_C|Gethud_widget (Variables|Default|GetPlayer_Character_BP))) (/ (Variables|Experience|GetXP) (Variables|Experience|GetMax_XP)))
  (Rendering|Components|TextRender|SetText (Variables|/Game/UI/WB_HUD.WB_HUD_C|GetExperienceText (Variables|/Game/ThirdPerson/Blueprints/BP_ThirdPersonCharacter.BP_ThirdPersonCharacter_C|Gethud_widget (Variables|Default|GetPlayer_Character_BP))) (Utilities|Text|FormatText "{Current XP} / {Max XP}" (Variables|Experience|GetXP) (Variables|Experience|GetMax_XP)))
  (Rendering|Components|TextRender|SetText (Variables|/Game/UI/WB_HUD.WB_HUD_C|GetLevel_Text (Variables|/Game/ThirdPerson/Blueprints/BP_ThirdPersonCharacter.BP_ThirdPersonCharacter_C|Gethud_widget (Variables|Default|GetPlayer_Character_BP))) (Utilities|Text|ToText(Integer) (Variables|Experience|GetLevel))))

(event EventTick
  (params (DeltaSeconds :type Float%20%28single-precision%29)))

(fn DecreaseHealth
  (params (Damage :type Float%20%28double-precision%29))
  (bind _player_character_bp (Variables|Default|GetPlayer_Character_BP))
  (bind _hud_widget (Variables|/Game/ThirdPerson/Blueprints/BP_ThirdPersonCharacter.BP_ThirdPersonCharacter_C|Gethud_widget _player_character_bp))
  (if (not (<= (Variables|Health|GetCurrent_Health) 0.0))
    (bind _output_get (Variables|Health|SetCurrent_Health (- (Variables|Health|GetCurrent_Health) Damage)))
    (Progress|SetPercent (Variables|/Game/UI/WB_HUD.WB_HUD_C|GetHealth_Bar _hud_widget) (/ _output_get (Variables|Health|GetMax_Health)))
    (Rendering|Components|TextRender|SetText (Variables|/Game/UI/WB_HUD.WB_HUD_C|GetHealth_Text _hud_widget) (Utilities|Text|ToText(Float) (Variables|Health|GetCurrent_Health) "HalfToEven"))
    (if (<= (Variables|Health|GetCurrent_Health) 0.0)
      _
      (else
        (return false))))
  (return true))

(fn IncreaseMaxHealth
  (params (health_incremention :type Float%20%28double-precision%29))
  (bind _player_character_bp (Variables|Default|GetPlayer_Character_BP))
  (bind _hud_widget (Variables|/Game/ThirdPerson/Blueprints/BP_ThirdPersonCharacter.BP_ThirdPersonCharacter_C|Gethud_widget _player_character_bp))
  (Variables|Health|SetMax_Health (+ (Variables|Health|GetMax_Health) health_incremention))
  (Progress|SetPercent (Variables|/Game/UI/WB_HUD.WB_HUD_C|GetHealth_Bar _hud_widget) (/ (Variables|Health|GetCurrent_Health) (Variables|Health|GetMax_Health)))
  (Rendering|Components|TextRender|SetText (Variables|/Game/UI/WB_HUD.WB_HUD_C|GetHealth_Text _hud_widget) (Utilities|Text|ToText(Float) (Variables|Health|GetCurrent_Health) "HalfToEven")))

(fn DecreaseStamina
  (params (stamina_depleted :type Float%20%28double-precision%29))
  (if (not (<= (Variables|Stamina|GetCurrent_Stamina) 0.0))
    (Variables|Stamina|SetCurrent_Stamina (- (Variables|Stamina|GetCurrent_Stamina) stamina_depleted))
    (Progress|SetPercent (Variables|/Game/UI/WB_HUD.WB_HUD_C|GetStamina_Bar (Variables|/Game/ThirdPerson/Blueprints/BP_ThirdPersonCharacter.BP_ThirdPersonCharacter_C|Gethud_widget (Variables|Default|GetPlayer_Character_BP))) (/ (Variables|Stamina|GetCurrent_Stamina) (Variables|Stamina|GetMax_Stamina)))
    (if (<= (Variables|Stamina|GetCurrent_Stamina) 0.0)
      _
      (else
        (return false))))
  (return true))

(fn IncreaseMaxStamina
  (params (added_stamina :type Float%20%28double-precision%29))
  (Variables|Stamina|SetMax_Stamina (+ (Variables|Stamina|GetMax_Stamina) added_stamina))
  (Progress|SetPercent (Variables|/Game/UI/WB_HUD.WB_HUD_C|GetStamina_Bar (Variables|/Game/ThirdPerson/Blueprints/BP_ThirdPersonCharacter.BP_ThirdPersonCharacter_C|Gethud_widget (Variables|Default|GetPlayer_Character_BP))) (/ (Variables|Stamina|GetCurrent_Stamina) (Variables|Stamina|GetMax_Stamina))))

(fn IncreaseHealth
  (params (added_health :type Float%20%28double-precision%29))
  (bind _player_character_bp (Variables|Default|GetPlayer_Character_BP))
  (bind _hud_widget (Variables|/Game/ThirdPerson/Blueprints/BP_ThirdPersonCharacter.BP_ThirdPersonCharacter_C|Gethud_widget _player_character_bp))
  (Variables|Health|SetCurrent_Health (+ (Variables|Health|GetCurrent_Health) added_health))
  (if (> (Variables|Health|GetCurrent_Health) (Variables|Health|GetMax_Health))
    (Variables|Health|SetCurrent_Health (Variables|Health|GetMax_Health)))
  (Progress|SetPercent (Variables|/Game/UI/WB_HUD.WB_HUD_C|GetHealth_Bar _hud_widget) (/ (Variables|Health|GetCurrent_Health) (Variables|Health|GetMax_Health)))
  (Rendering|Components|TextRender|SetText (Variables|/Game/UI/WB_HUD.WB_HUD_C|GetHealth_Text _hud_widget) (Utilities|Text|ToText(Float) (Variables|Health|GetCurrent_Health) "HalfToEven")))

(fn IncreaseStamina
  (params (added_stamina :type Float%20%28double-precision%29))
  (Variables|Stamina|SetCurrent_Stamina (+ (Variables|Stamina|GetCurrent_Stamina) added_stamina))
  (if (> (Variables|Stamina|GetCurrent_Stamina) (Variables|Stamina|GetMax_Stamina))
    (Variables|Stamina|SetCurrent_Stamina (Variables|Stamina|GetMax_Stamina)))
  (Progress|SetPercent (Variables|/Game/UI/WB_HUD.WB_HUD_C|GetStamina_Bar (Variables|/Game/ThirdPerson/Blueprints/BP_ThirdPersonCharacter.BP_ThirdPersonCharacter_C|Gethud_widget (Variables|Default|GetPlayer_Character_BP))) (/ (Variables|Stamina|GetCurrent_Stamina) (Variables|Stamina|GetMax_Stamina))))

(fn IncreaseXP
  (params (Added%20Experience :type Float%20%28double-precision%29))
  (Variables|Experience|SetXP (+ (Variables|Experience|GetXP) Added%20Experience))
  (if (>= (Variables|Experience|GetXP) (Variables|Experience|GetMax_XP))
    (LevelAndXP|IncreaseLevel 1))
  (Progress|SetPercent (Variables|/Game/UI/WB_HUD.WB_HUD_C|GetExperienceBar (Variables|/Game/ThirdPerson/Blueprints/BP_ThirdPersonCharacter.BP_ThirdPersonCharacter_C|Gethud_widget (Variables|Default|GetPlayer_Character_BP))) (/ (Variables|Experience|GetXP) (Variables|Experience|GetMax_XP)))
  (Rendering|Components|TextRender|SetText (Variables|/Game/UI/WB_HUD.WB_HUD_C|GetExperienceText (Variables|/Game/ThirdPerson/Blueprints/BP_ThirdPersonCharacter.BP_ThirdPersonCharacter_C|Gethud_widget (Variables|Default|GetPlayer_Character_BP))) (Utilities|Text|FormatText "{Current XP} / {Max XP}" (Variables|Experience|GetXP) (Variables|Experience|GetMax_XP))))

(fn IncreaseLevel
  (params (Added%20Level :type Integer))
  (Variables|Experience|SetLevel (+ (Variables|Experience|GetLevel) Added%20Level))
  (Variables|Experience|SetMax_XP (+ (Variables|Experience|GetMax_XP) 1.5e+02))
  (Variables|Experience|SetXP 0.0)
  (Rendering|Components|TextRender|SetText (Variables|/Game/UI/WB_HUD.WB_HUD_C|GetLevel_Text (Variables|/Game/ThirdPerson/Blueprints/BP_ThirdPersonCharacter.BP_ThirdPersonCharacter_C|Gethud_widget (Variables|Default|GetPlayer_Character_BP))) (Utilities|Text|ToText(Integer) (Variables|Experience|GetLevel))))