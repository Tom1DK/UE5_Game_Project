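; Melee combat component for BP_ThirdPersonCharacter that plays a four-step sword and kick combo from the attack input.
; Input during an attack is buffered in SaveAttack, and Sword_Attack_Combo either plays the next AttackIndex montage or resets the combo.
; A looping-timer sphere trace along the blade and a one-shot sphere trace for stab and kick damage "Damagable"-tagged actors, adding camera shake, blood and sound.
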(event Custom|Sword_Attack
  ;[1 1 1] Combo System
  ;;[1 1 1] Sword Attack
  (if (Variables|Default|Getis_attacking?)
    (Variables|Default|Setsave_attack? true)
    (else
      (Variables|Default|Setis_attacking? true)
      (switch int (Variables|Default|Getattack_index)
        (:0
          (CallFunction|Attack1))
        (:1
          (CallFunction|Attack2))
        (:2
          (CallFunction|Attack3))
        (:3
          (CallFunction|Attack4))))))

(event Custom|Sword_Attack_Combo
  ;[1 1 1] Combo System
  ;;[1 1 1] Combo Count
  (if (Variables|Default|Getsave_attack?)
    (Variables|Default|Setsave_attack? false)
    (switch int (Variables|Default|Getattack_index)
      (:0
        (CallFunction|Attack1))
      (:1
        (CallFunction|Attack2))
      (:2
        (CallFunction|Attack3))
      (:3
        (CallFunction|Attack4)))
    (else
      (CallFunction|StopCombo))))

(event Custom|Attack_2
  ;[1 1 1] Combo System
  ;;[1 1 1] Attack 2
  (Utilities|FlowControl|DoOnce false :!label _label
    (:Completed
      (Utilities|FlowControl|Delay 0.5)
      (Animation|Montage|PlayMontage (Variables|Default|Getcharacter_mesh) "/Game/Characters/RPG_Character/Animations/Sword_Attacks/Attack2_Montage.Attack2_Montage"
        (:then
          (Variables|Default|Setattack_index 2)
          (goto _label Reset))))))

(event Custom|Play_Sword_Hit_Sound
  ;[1 1 1] Sound Effects
  (Audio|PlaySoundatLocation "/Game/Audio/Sword-Hits/MS_Sword_Hit.MS_Sword_Hit" (Transformation|GetActorLocation (Components|GetOwner)) "0, 0, 0" 1.0 1.0 0.0 0 0 0 0))

(event Custom|Attack_3
  ;[1 1 1] Combo System
  ;;[1 1 1] Attack 3
  (Utilities|FlowControl|DoOnce false :!label _label
    (:Completed
      (Utilities|FlowControl|Delay 0.45)
      (Animation|Montage|PlayMontage (Variables|Default|Getcharacter_mesh) "/Game/Characters/RPG_Character/Animations/Sword_Attacks/Kick_Montage.Kick_Montage"
        (:then
          (Variables|Default|Setattack_index 3)
          (goto _label Reset))))))

(event Custom|Stop_Combo
  ;[1 1 1] Combo System
  ;;[1 1 1] Stop Combo/Attack
  (Variables|Default|Setis_attacking? false)
  (Variables|Default|Setattack_index 0))

(event Custom|Attack_4
  ;[1 1 1] Combo System
  ;;[1 1 1] Attack 4
  (Utilities|FlowControl|DoOnce false :!label _label
    (:Completed
      (Utilities|FlowControl|Delay 0.4)
      (Animation|Montage|PlayMontage (Variables|Default|Getcharacter_mesh) "/Game/Characters/RPG_Character/Animations/Sword_Attacks/Attack3_Montage.Attack3_Montage"
        (:then
          (Variables|Default|Setattack_index 4)
          (goto _label Reset))))))

(event Custom|Start_Sword_Trace
  ;[1 1 1] Sword Trace 1/4
  (bind _returnvalue (Utilities|Time|SetTimerbyEvent (delegate Custom|Sword_Trace_Loop) 0.01 true))
  (Variables|Default|Setsword_trace_loop_var _returnvalue))

(event Custom|Sword_Trace_Loop
  ;[1 1 1] Sword Trace 1/4
  (bind (_outhit _returnvalue) (Collision|SphereTraceByChannel (Transformation|GetWorldLocation (Variables|/Game/ThirdPerson/Blueprints/BP_ThirdPersonCharacter.BP_ThirdPersonCharacter_C|GetSword%20Top%20Point (Variables|Default|Getcharacter_bp))) (Transformation|GetWorldLocation (Variables|/Game/ThirdPerson/Blueprints/BP_ThirdPersonCharacter.BP_ThirdPersonCharacter_C|GetSword%20Bottom%20Point (Variables|Default|Getcharacter_bp))) 12.0 "TraceTypeQuery1" false 0 "ForDuration" true "(R=1.000000,G=0.000000,B=0.000000,A=1.000000)" "(R=0.000000,G=1.000000,B=0.000000,A=1.000000)" 1.0))
  (if _returnvalue
    (if (Actor|ActorHasTag (.HitActor (Collision|BreakHitResult _outhit)) "Damagable")
      (Utilities|FlowControl|DoOnce false :!label _label
        (:Completed
          (Game|Damage|ApplyDamage (.HitActor (Collision|BreakHitResult _outhit)) 2.0 0 0)
          (Camera|PlayWorldCameraShake "/Game/Blueprints/BP_Sword_Hit_Camera_Shake.BP_Sword_Hit_Camera_Shake_C" (.Location (Collision|BreakHitResult _outhit)) 0.0 2e+03)
          (CallFunction|PlaySwordHitSound)
          (Effects|SpawnEmitteratLocation "/Game/VFX/Particles/Blood/P_Blood_Splat_Cone.P_Blood_Splat_Cone" (.Location (Collision|BreakHitResult _outhit)) (Math|Rotator|MakeRotfromXY (.Normal (Collision|BreakHitResult _outhit)) (.Normal (Collision|BreakHitResult _outhit))) "2.000000,2.000000,2.000000" true "AutoRelease")
          (Utilities|FlowControl|Delay 0.5)
          (goto _label Reset))))))

(event Custom|Stop_Sword_Trace
  ;[1 1 1] Sword Trace 1/4
  (Utilities|Time|ClearandInvalidateTimerbyHandle (Variables|Default|Getsword_trace_loop_var)))

(event Custom|Sphere_trace
  (bind _character_bp (Variables|Default|Getcharacter_bp))
  (bind _sphere_trace (Variables|/Game/ThirdPerson/Blueprints/BP_ThirdPersonCharacter.BP_ThirdPersonCharacter_C|GetSphere%20Trace _character_bp))
  (bind _returnvalue (Transformation|GetWorldLocation _sphere_trace))
  ;[1 1 1] Sphere Trace (For Stab and Kick) 2/3
  (bind (_outhit _returnvalue_2) (Collision|SphereTraceByChannel _returnvalue _returnvalue 1.5e+02 "TraceTypeQuery1" false 0 "ForDuration" true "(R=1.000000,G=0.000000,B=0.000000,A=1.000000)" "(R=0.000000,G=1.000000,B=0.000000,A=1.000000)" 1.0))
  (if _returnvalue_2
    (if (Actor|ActorHasTag (.HitActor (Collision|BreakHitResult _outhit)) "Damagable")
      (Game|Damage|ApplyDamage (.HitActor (Collision|BreakHitResult _outhit)) 1.0 0 0)
      (Camera|PlayWorldCameraShake "/Game/Blueprints/BP_Sword_Hit_Camera_Shake.BP_Sword_Hit_Camera_Shake_C" (.Location (Collision|BreakHitResult _outhit)) 0.0 2e+03)
      (CallFunction|KickHitSound)
      (Effects|SpawnEmitteratLocation "/Game/VFX/Particles/Blood/P_Blood_Splat_Cone.P_Blood_Splat_Cone" (.Location (Collision|BreakHitResult _outhit)) (Math|Rotator|MakeRotfromXY (.Normal (Collision|BreakHitResult _outhit)) (.Normal (Collision|BreakHitResult _outhit))) "2.000000,2.000000,2.000000" true "AutoRelease"))))

(event Custom|Attack_1
  ;[1 1 1] Combo System
  ;;[1 1 1] Attack 1
  (Utilities|FlowControl|DoOnce false :!label _label
    (:Completed
      (Utilities|FlowControl|Delay 0.1)
      (Animation|Montage|PlayMontage (Variables|Default|Getcharacter_mesh) "/Game/Characters/RPG_Character/Animations/Sword_Attacks/Attack1_Montage.Attack1_Montage"
        (:then
          (Variables|Default|Setattack_index 1)
          (goto _label Reset))))))

(event Custom|Kick_Hit_sound
  ;[1 1 1] Sound Effects
  (Audio|PlaySoundatLocation "/Game/Audio/Sword-Hits/Kick.Kick" (Transformation|GetActorLocation (Components|GetOwner)) "0, 0, 0" 1.0 1.0 0.0 0 0 0 0))

(event Input|EnhancedActionEvents|EnhancedInputActionIA_Attack
  (params (ActionValue :type Boolean) (ElapsedSeconds :type Float%20%28double-precision%29) (TriggeredSeconds :type Float%20%28double-precision%29) (InputAction :type Input%20Action%20Object%20Reference :default "/Game/ThirdPerson/Input/Actions/IA_Attack.IA_Attack"))
  ;[1 1 1] Combo System
  ;;[1 1 1] Attack Input
  (:Started
    (if (Variables|Default|Getcan_attack?)
      (CallFunction|SwordAttack))))

(event EventBeginPlay
  ;[1 1 1] Combo System
  (bind _asbp_third_person_character (Utilities|Casting|CastToBP_ThirdPersonCharacter (Components|GetOwner)))
  (Variables|Default|Setcharacter_bp _asbp_third_person_character)
  (Variables|Default|Setcharacter_mesh (Variables|/Script/Engine.Character|GetMesh _asbp_third_person_character)))