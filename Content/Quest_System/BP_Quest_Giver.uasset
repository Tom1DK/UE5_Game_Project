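; BP_Quest_Giver is a quest giver actor that the player interacts with to open a quest UI.
; Its trigger radius shows an interact prompt for the third-person character, and Tick rotates that prompt toward the camera.
; Interact creates WB_Quest_Giver with cursor and Game-and-UI input, or removes it once WidgetActive is set.
; The close branch leaves the cursor shown, and its input-mode and WidgetActive resets are unconnected, so the widget cannot reopen.
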(event OnComponentBeginOverlap(Quest_Trigger_Radius)
  (params (OverlappedComponent :type Primitive%20Component%20Object%20Reference) (OtherActor :type Actor%20Object%20Reference) (OtherComp :type Primitive%20Component%20Object%20Reference) (OtherBodyIndex :type Integer) (bFromSweep :type Boolean) (SweepResult :type Hit%20Result%20Structure%20%28by%20ref%29))
  (Utilities|Casting|CastToBP_ThirdPersonCharacter OtherActor)
  (Rendering|SetVisibility (Variables|Default|GetInteract_Widget) true false))

(event OnComponentEndOverlap(Quest_Trigger_Radius)
  (params (OverlappedComponent :type Primitive%20Component%20Object%20Reference) (OtherActor :type Actor%20Object%20Reference) (OtherComp :type Primitive%20Component%20Object%20Reference) (OtherBodyIndex :type Integer))
  (Utilities|Casting|CastToBP_ThirdPersonCharacter OtherActor)
  (Rendering|SetVisibility (Variables|Default|GetInteract_Widget) false false))

(event Collision|EventActorBeginOverlap
  (params (OtherActor :type Actor%20Object%20Reference)))

(event EventTick
  (params (DeltaSeconds :type Float%20%28single-precision%29))
  (Transformation|SetWorldRotation (Variables|Default|GetInteract_Widget) (Math|Rotator|FindLookatRotation (Transformation|GetWorldLocation (Variables|Default|GetInteract_Widget)) (Transformation|GetWorldLocation (Variables|/Script/Engine.PlayerCameraManager|GetTransformComponent (Game|GetPlayerCameraManager 0)))) false false))

(event EventInteract
  (bind _returnvalue (Game|GetPlayerController 0))
  (if (not (Variables|Default|Getwidget_active))
    (bind _returnvalue_2 (UserInterface|CreateWidget "/Game/Quest_System/WB_Quest_Giver.WB_Quest_Giver_C"))
    (bind _output_get (Variables|Default|Setquests_widget _returnvalue_2))
    (UserInterface|Viewport|AddtoViewport _output_get 0)
    (Variables|Default|Setwidget_active true)
    (Variables|/Script/Engine.PlayerController|SetbShowMouseCursor _returnvalue true)
    (Input|SetInputModeGameandUI _returnvalue (Variables|Default|Getquests_widget) "DoNotLock" true false)
    (else
      (Widget|RemovefromParent (Variables|Default|Getquests_widget))
      (Variables|Default|Setquests_widget 0)
      (Variables|/Script/Engine.PlayerController|SetbShowMouseCursor (Game|GetPlayerController 0) true))))

(fn ConstructionScript)