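; BPC_Quest is a quest component that drives the on-screen quest HUD for the active quest.
; On BeginPlay it creates the WB_Quest_HUD widget, stores it and adds it to the viewport.
; Two custom events push the active quest's name into the HUD text and pass its objectives to the widget's FillObjectives to populate the list.
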(event Custom|Set_Active_Quest_Text
  (Rendering|Components|TextRender|SetText (Variables|/Game/UI/WB_Quest_HUD.WB_Quest_HUD_C|GetActiveQuest (Variables|Default|Getquest_hud_widget)) (Utilities|Text|ToText(String) (.Name (Utilities|Struct|BreakS_Quest (Variables|Default|Getactive_quest))))))

(event Custom|Set_Objectives
  (Default|FillObjectives (Variables|Default|Getquest_hud_widget) (.objectives (Variables|Default|Getactive_quest))))

(event EventBeginPlay
  (bind _returnvalue (UserInterface|CreateWidget "/Game/UI/WB_Quest_HUD.WB_Quest_HUD_C"))
  (bind _output_get (Variables|Default|Setquest_hud_widget _returnvalue))
  (UserInterface|Viewport|AddtoViewport _output_get 0))