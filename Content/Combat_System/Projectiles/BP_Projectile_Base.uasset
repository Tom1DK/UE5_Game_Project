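; Base projectile actor for the combat system, with configurable speed, gravity, optional homing and impact effects.
; The construction script applies these settings to ProjectileMovement and homes on the target's root component when enabled.
; On BeginPlay it ignores its owner in movement collision and aims its velocity at any valid target.
; A box hit calls OnProjectileImpact for external handling, spawns the impact particle and sound, then destroys the projectile.
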(event OnComponentHit(BoxCollision)
  (params (HitComponent :type Primitive%20Component%20Object%20Reference) (OtherActor :type Actor%20Object%20Reference) (OtherComp :type Primitive%20Component%20Object%20Reference) (NormalImpulse :type Vector :default "0, 0, 0") (Hit :type Hit%20Result%20Structure%20%28by%20ref%29))
  (bind _location (Collision|BreakHitResult Hit))
  (Default|CallOnProjectileImpact OtherActor Hit)
  (Effects|SpawnEmitteratLocation (Variables|ProjectileSettings|Getimpact_effect) _location "0, 0, 0" (Variables|ProjectileSettings|Getimpact_size))
  (Audio|PlaySoundatLocation (Variables|ProjectileSettings|GetImpact_sound) _location "0, 0, 0" 1.0 1.0 0.0 0 0 0 0)
  ;[1 1 1] Might Remove/Also in Attack System
  (Collision|IgnoreActorwhenMoving (Variables|Default|GetBox%20Collision) (Components|GetOwner) true)
  (Actor|DestroyActor))

(event Custom|Rotate_to_Target
  (Variables|/Script/Engine.MovementComponent|SetVelocity (Variables|Default|GetProjectileMovement) (* (Math|Vector|GetUnitDirection(Vector) (Transformation|GetActorLocation) (Transformation|GetActorLocation (Variables|ProjectileSettings|Gethas_target))) (Variables|ProjectileSettings|Getspeed))))

(event EventBeginPlay
  (Collision|IgnoreActorwhenMoving (Variables|Default|GetBox%20Collision) (Components|GetOwner) true)
  (Variables|ProjectileSettings|Gethas_target
    (:then
      (CallFunction|RotatetoTarget))
    (:else)))

(fn ConstructionScript
  (bind _projectilemovement (Variables|Default|GetProjectileMovement))
  (Variables|/Script/Engine.ProjectileMovementComponent|SetInitialSpeed _projectilemovement (Variables|ProjectileSettings|Getspeed))
  (Variables|/Script/Engine.ProjectileMovementComponent|SetMaxSpeed _projectilemovement (Variables|ProjectileSettings|Getspeed))
  (Variables|/Script/Engine.ProjectileMovementComponent|SetProjectileGravityScale _projectilemovement (Variables|ProjectileSettings|Getgravity))
  (Variables|ProjectileSettings|Gethas_target
    (:then
      (if (Variables|ProjectileSettings|Getis_homing)
        (Variables|/Script/Engine.ProjectileMovementComponent|SetbIsHomingProjectile _projectilemovement true)
        (Variables|/Script/Engine.ProjectileMovementComponent|SetHomingTargetComponent _projectilemovement (Variables|/Script/Engine.Actor|GetRootComponent (Variables|ProjectileSettings|Gethas_target)))))
    (:else)))