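; Attack component that carries out combat moves for its owner: arrow shot, lightning strike, fireball, dark orb and area heal.
; Arrows use a pawn line trace, while spells spawn projectile or AOE actors and bind their impact or overlap events to damage or healing.
; Arrow and projectile hits also report damage events, with projectile hits signalling attack end.
; The heal AOE spawns at a downward trace hit and heals only its intended target.
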(event Custom|Dark_Orb_Barrage
  (params (SpawnTransform :type Transform) (has_target :type Actor%20Object%20Reference) (damage_info :type S%20Damage%20Info%20Structure) (spell_to_cast :type Boolean))
  (bind _returnvalue (Game|SpawnActorfromClass "/Game/Combat_System/Projectiles/BP_Projectiles_Base_Dark_Orb.BP_Projectiles_Base_Dark_Orb_C" SpawnTransform "Undefined" "MultiplyWithRoot" (Components|GetOwner) 1.4e+03 0.001 has_target false 0))
  (EventDispatchers|BindEventtoOnProjectileImpact _returnvalue (delegate Custom|On_Dark_Orb_Hit))
  ;[1 1 1] Self Damage
  (Collision|IgnoreActorwhenMoving (Actor|GetComponentbyClass (Components|GetOwner) "/Script/Engine.CapsuleComponent") _returnvalue true))

(event Custom|On_Dark_Orb_Hit
  (params (other_actor :type Actor%20Object%20Reference) (hit :type Hit%20Result%20Structure))
  (bind _returnvalue (Components|GetOwner))
  (Class|BPIDamagable|TakeDamage(Message) other_actor (stale Custom|Dark_Orb_Barrage damage_info) _returnvalue)
  (Class|AISenseDamage|ReportDamageEvent other_actor _returnvalue (.Damage_Amount (Utilities|Struct|BreakS_Damage_Info (stale Custom|Dark_Orb_Barrage damage_info))) (Transformation|GetActorLocation _returnvalue) "0, 0, 0" "None")
  (Default|CallOnAttackEnded))

(event Custom|Fireball
  (params (SpawnTransform :type Transform) (has_target :type Actor%20Object%20Reference) (damage_info :type S%20Damage%20Info%20Structure) (spell_to_cast :type Boolean))
  ;[1 1 1 1 62] Fireball
  (bind _returnvalue (Game|SpawnActorfromClass "/Game/Combat_System/Projectiles/BP_Projectiles_Base_Fireball.BP_Projectiles_Base_Fireball_C" SpawnTransform "Undefined" "MultiplyWithRoot" (Components|GetOwner) 5e+02 0.001 has_target false 0))
  (EventDispatchers|BindEventtoOnProjectileImpact _returnvalue (delegate Custom|On_Fireball_Hit))
  ;;[1 1 1] Self Damage
  (Collision|IgnoreActorwhenMoving (Actor|GetComponentbyClass (Components|GetOwner) "/Script/Engine.CapsuleComponent") _returnvalue true))

(event Custom|On_Fireball_Hit
  (params (other_actor :type Actor%20Object%20Reference) (hit :type Hit%20Result%20Structure))
  (bind _returnvalue (Components|GetOwner))
  ;[1 1 1 1 62] Fireball
  (Class|BPIDamagable|TakeDamage(Message) other_actor (stale Custom|Fireball damage_info) _returnvalue)
  (Class|AISenseDamage|ReportDamageEvent other_actor _returnvalue (.Damage_Amount (Utilities|Struct|BreakS_Damage_Info (stale Custom|Fireball damage_info))) (Transformation|GetActorLocation _returnvalue) "0, 0, 0" "None")
  (Default|CallOnAttackEnded))

(event Custom|Shoot_Arrow
  (params (trace_start :type Vector) (trace_end :type Vector) (damage_info :type S%20Damage%20Info%20Structure))
  (bind _returnvalue (Components|GetOwner))
  ;[1 1 1 1 62] Shoot Arrow
  (bind (_outhit _returnvalue_2) (Collision|LineTraceForObjects trace_start trace_end (Utilities|Array|MakeArray "ObjectTypeQuery3") false 0 "None"))
  (if _returnvalue_2
    (Class|BPIDamagable|TakeDamage(Message) (.HitActor (Collision|BreakHitResult _outhit)) damage_info _returnvalue)
    (Class|AISenseDamage|ReportDamageEvent (.HitActor (Collision|BreakHitResult _outhit)) _returnvalue (.Damage_Amount (Utilities|Struct|BreakS_Damage_Info damage_info)) (Transformation|GetActorLocation _returnvalue) "0, 0, 0" "None")))

(event Custom|Damage_Enemy_AOE
  (params (actor :type Actor%20Object%20Reference))
  ;[1 1 1 1 62] Lightning Strike
  (Class|BPIDamagable|TakeDamage(Message) actor (Utilities|Struct|MakeS_Damage_Info 12.0 "NewEnumerator3" "NewEnumerator1")))

(event Custom|Lightning_Strike
  (params (attack_target :type Actor%20Object%20Reference))
  (bind _returnvalue (Components|GetOwner))
  (bind (_aspawn _bsuccess) (Utilities|Casting|CastToPawn _returnvalue))
  ;[1 1 1 1 62] Lightning Strike
  (bind _returnvalue_2 (Game|SpawnActorfromClass "/Game/Combat_System/AOE/BP_AOE_Lightning_Strike.BP_AOE_Lightning_Strike_C" (Math|Transform|MakeTransform "0, 0, 0" "0, 0, 0" "1.000000,1.000000,1.000000") "Undefined" "MultiplyWithRoot" 0 attack_target 1.0 1.5e+02 true false false (select _bsuccess _aspawn 0)))
  (EventDispatchers|AssignOnAOEOverlapActor _returnvalue_2 (delegate Custom|Damage_Enemy_AOE)))

(event Custom|Heal_Target_AOE
  (params (heal_target :type Actor%20Object%20Reference))
  (bind _returnvalue (Transformation|GetActorLocation heal_target))
  ;[1 1 1 1 62] Heal: HOT
  (Utilities|IsValid heal_target
    (:Is%20Valid
      (bind (_outhit _returnvalue_2) (Collision|LineTraceByChannel _returnvalue (* _returnvalue "1.000000,1.000000,-1000.000000") "TraceTypeQuery1" false (Utilities|Array|MakeArray heal_target) "None"))
      (if _returnvalue_2
        (bind _returnvalue_3 (Game|SpawnActorfromClass "/Game/Combat_System/AOE/BP_AOE_Heal.BP_AOE_Heal_C" (Math|Transform|MakeTransform (.Location (Collision|BreakHitResult _outhit)) "0, 0, 0" "1.000000,1.000000,1.000000") "Undefined" "MultiplyWithRoot" 0 1.0 1e+01 1.2e+02 false false false 0))
        (EventDispatchers|BindEventtoOnAOEOverlapActor _returnvalue_3 (delegate Custom|On_Heal_Target))
        (Default|Trigger _returnvalue_3)))))

(event Custom|On_Heal_Target
  (params (actor :type Actor%20Object%20Reference))
  ;[1 1 1 1 62] Heal: HOT
  (if (== actor (stale Custom|Heal_Target_AOE heal_target))
    (Class|BPIDamagable|Heal(Message) actor 2.0)))