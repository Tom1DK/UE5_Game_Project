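; Base Blueprint for area-of-effect blasts that adds visual and audio feedback to the inherited Trigger behavior.
; Trigger calls the parent, then spawns the blast particle effect attached to the root and plays the blast sound at the actor's location.
; The actor destroys itself when the particle system finishes, or after a short delay if no effect is set.
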(event Custom|OnSystemFinished_Event
  (params (PSystem :type Particle%20System%20Component%20Object%20Reference))
  (Actor|DestroyActor))

(event Custom|Spawn_Blast_Effect
  (bind _blast_effect (Variables|Default|Getblast_effect)
    (:then
      (bind _returnvalue (Effects|SpawnEmitterAttached _blast_effect (Variables|Default|GetDefaultSceneRoot) "None"))
      (EventDispatchers|AssignOnSystemFinished _returnvalue (delegate Custom|OnSystemFinished_Event)))
    (:else
      (Utilities|FlowControl|Delay 1.0)
      (Actor|DestroyActor))))

(event Custom|Play_Blast_Sound
  (bind _blast_sound (Variables|Default|Getblast_sound)
    (:then
      (Audio|PlaySoundatLocation _blast_sound (Transformation|GetActorLocation) "0, 0, 0" 1.0 1.0 0.0 0 0 0 0))
    (:else)))

(event EventTrigger
  (|CallParentFunction)
  (CallFunction|SpawnBlastEffect)
  (CallFunction|PlayBlastSound))

(fn ConstructionScript
  (|CallParentFunction))