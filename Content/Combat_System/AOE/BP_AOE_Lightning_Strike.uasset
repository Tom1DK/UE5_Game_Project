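; Lightning strike AOE attack actor that marks the ground with a magic circle decal before striking.
; On BeginPlay it traces from AttackTarget toward an end point made by scaling the target's Z by -1000, then moves to any hit.
; It spawns the decal there, waits DelayBeforeStrike, calls Trigger and destroys the decal.
; The strike effect itself lies in Trigger, which is not defined in this graph.
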(event Custom|Move_to_Floor
  (bind _attack_target (Variables|AOESettings|Getattack_target)
    (:then
      (bind (_outhit _returnvalue) (Collision|LineTraceByChannel (Transformation|GetActorLocation _attack_target) (* (Transformation|GetActorLocation _attack_target) "1.000000,1.000000,-1000.000000") "TraceTypeQuery1" false (Utilities|Array|MakeArray _attack_target) "None"))
      (if _returnvalue
        (Transformation|SetActorLocation (.Location (Collision|BreakHitResult _outhit)) false false)))
    (:else)))

(event EventBeginPlay
  (|CallParentFunction)
  (CallFunction|MovetoFloor)
  (bind _returnvalue (Rendering|Decal|SpawnDecalatLocation "/Game/Combat_System/AOE/Decals/M_Magic_Circle_Inst.M_Magic_Circle_Inst" "10.000000,150.000000,150.000000" (Transformation|GetActorLocation) "-90.000000,0.000000,0.000000" 0.0))
  (Utilities|FlowControl|Delay (Variables|AOESettings|Getdelay_before_strike))
  (CallFunction|Trigger)
  (Utilities|IsValid _returnvalue
    (:Is%20Valid
      (Components|DestroyComponent _returnvalue))))

(fn ConstructionScript
  (|CallParentFunction))