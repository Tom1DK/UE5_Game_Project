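; BP_Base_AOE is a base area-of-effect actor for the combat system that detects pawns within a radius of its location.
; It can trigger itself one second after BeginPlay or through its Trigger event.
; The trigger runs a sphere overlap, optionally ignoring the instigator and drawing a debug sphere.
; Each hit actor is broadcast through the OnAOEOverlapActor dispatcher and printed, leaving the effect itself to listeners.
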(event Custom|Spawn_AOE_Sphere
  (if (Variables|AOESettings|Getdraw_debug_sphere)
    (Rendering|Debug|DrawDebugSphere (Transformation|GetActorLocation) (Variables|AOESettings|Getradius) 12 "(R=1.000000,G=1.000000,B=1.000000,A=1.000000)" 2.0 1.0))
  (bind _outactors (Collision|SphereOverlapActors (Transformation|GetActorLocation) (Variables|AOESettings|Getradius) (Utilities|Array|MakeArray "ObjectTypeQuery3") 0 (select (Variables|AOESettings|Getignore_instigator) (Utilities|Array|MakeArray (Game|GetInstigator)) 0)))
  (for _array_element _outactors
    (Default|CallOnAOEOverlapActor _array_element)
    (Development|PrintString (Utilities|GetDisplayName _array_element))))

(event Custom|Trigger
  (CallFunction|SpawnAOESphere))

(event EventBeginPlay
  (if (Variables|AOESettings|Gettrigger_on_begin_play)
    (Utilities|FlowControl|Delay 1.0)
    (CallFunction|Trigger)))

(fn ConstructionScript)