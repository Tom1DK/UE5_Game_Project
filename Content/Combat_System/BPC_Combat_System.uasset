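; Combat component that manages health, damage, blocking and death for its owner.
; TakeDamage uses Can_Be_Damaged to route hits to block, damage or no damage from invincibility, death, blocking and damage-info flags.
; It fires blocked, death or damage-response events, returning true only when damage kills or interrupts.
; Heal restores health up to the maximum while the owner is alive.
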(event EventBeginPlay)

(event EventTick
  (params (DeltaSeconds :type Float%20%28single-precision%29)))

(fn Heal
  (params (amount_healed :type Float%20%28double-precision%29))
  (if (not (Variables|Default|Getis_dead))
    (bind _output_get (Variables|Default|Setcurrent_health (Math|Float|Clamp(Float) (+ amount_healed (Variables|Default|Getcurrent_health)) 0.0 (Variables|Default|Getmax_health))))
    (return _output_get)))

(fn TakeDamage
  (params (damage_info :type S%20Damage%20Info%20Structure))
  (bind (_damage_amount _damage_type _damage_response _is_blockable _is_parriable _force_unavoidable _force_interrupt) (Utilities|Struct|BreakS_Damage_Info damage_info))
  (Utilities|CanbeDamaged _force_unavoidable _is_blockable
    (:Block_Damage
      (Default|CallOnBlocked _is_parriable)
      (return false))
    (:Do_Damage
      (bind _output_get (Variables|Default|Setcurrent_health (- (Variables|Default|Getcurrent_health) _damage_amount)))
      (if (<= _output_get 0.0)
        (Variables|Default|Setis_dead true)
        (Default|CallOnDeath)
        (return true)
        (elif (or _force_interrupt (Variables|Default|Getis_interruptable))
          (Default|CallOnDamageResponse _damage_response)
          (return true))))
    (:No_Damage
      (return false))))